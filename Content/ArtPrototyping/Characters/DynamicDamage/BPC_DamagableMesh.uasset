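; Damage component that paints hit marks onto its owning BP_Character's parent skeletal mesh when that character takes damage.
; On BeginPlay it feeds a render target into the mesh's dynamic material as RT_Damage and creates an orthographic, show-only scene capture.
; Each hit briefly swaps material slot 0 to M_Unwrapper with hit location and radius, then captures additively into the target so marks accumulate.
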(event `self.ReceiveBeginPlay`
  (bind _mesh (`self.Mesh`))
  (bind _scenecapture (`self.SceneCapture`))
  (bind _returnvalue_location (`KismetMathLibrary.BreakTransform` (`self.K2_GetComponentToWorld` (`self.Mesh`))))
  (bind _asbp_character (cast `/Game/Characters/Blueprints/BP_Character` (`self.GetOwner`)))
  (add `/Game/Characters/Blueprints/BP_Character.OnTakeDamage` _asbp_character (delegate `OnHit`))
  (bind _asskeletal_mesh_component (cast `SkeletalMeshComponent` (`|GetArrayItem` (`self.GetParentComponents`)))
    (:`then`
      (set `self.Mesh` _asskeletal_mesh_component)
      (`|ExecutionSequence`
        (:`then_0`
          (bind _returnvalue (`KismetRenderingLibrary.CreateRenderTarget2D` 512 512))
          (set `self.RenderTarget` _returnvalue)
          (bind _returnvalue_2 (`PrimitiveComponent.CreateDynamicMaterialInstance` _mesh 0 (`PrimitiveComponent.GetMaterial` _mesh 0) "None"))
          (`PrimitiveComponent.SetMaterial` (`self.Mesh`) 0 _returnvalue_2)
          (`MaterialInstanceDynamic.SetTextureParameterValue` _returnvalue_2 "RT_Damage" (`self.RenderTarget`)))
        (:`then_1`
          (bind _returnvalue_3 (`|AddComponentByClass` :`self` (`self.GetOwner` self) :`Class` "/Script/Engine.SceneCaptureComponent2D"))
          (bind _output_get (set `self.SceneCapture` _returnvalue_3))
          (`self.K2_AttachToComponent` _output_get (`self.Mesh`) "None" "KeepWorld" "KeepWorld" "KeepWorld" false)
          (set `SceneCaptureComponent2D.OrthoWidth` 512.0 _scenecapture)
          (set `SceneComponent.bAbsoluteRotation` true _scenecapture)
          (set `SceneCaptureComponent2D.ProjectionType` "Orthographic" _scenecapture)
          (set `SceneCaptureComponent.PrimitiveRenderMode` "PRM_UseShowOnlyList" _scenecapture)
          (`self.K2_SetWorldTransform` _scenecapture (`KismetMathLibrary.MakeTransform` (+ _returnvalue_location (0.0 0.0 150.0)) (struct :`Pitch` -90.0 :`Yaw` -90.0)) false false)
          (`SceneCaptureComponent.ShowOnlyComponent` _scenecapture (`self.Mesh`))
          (set `SceneCaptureComponent2D.TextureTarget` (`self.RenderTarget`) _scenecapture)
          (set `SceneCaptureComponent.bCaptureEveryFrame` false _scenecapture)
          (set `SceneCaptureComponent.bCaptureOnMovement` false _scenecapture)
          (set `SceneCaptureComponent2D.CompositeMode` "SCCM_Additive" _scenecapture))
        (:`then_2`
          (`KismetSystemLibrary.Delay` 0.05)
          (`KismetRenderingLibrary.ClearRenderTarget2D` (`self.RenderTarget`)))))
    (:`CastFailed`
      (`KismetSystemLibrary.PrintString` "Warning: damagable mesh component not attached to skeletal mesh"))))

(event `OnHit`
  (params (Hit :type "HitResult Structure"))
  (`self.Paint` (`.Location` (`GameplayStatics.BreakHitResult` Hit)) 10.0 (make `Color` 255))
  (`KismetSystemLibrary.PrintString` "Hit damagabke"))

(event `Paint`
  (params (Location :type "Vector Structure") (Radius :type "Float (double-precision)") (Colour :type "Color Structure"))
  (bind _mesh (`self.Mesh`))
  (bind _mesh_2 (`self.Mesh`))
  (set `self.OldMat` (`PrimitiveComponent.GetMaterial` (`self.Mesh`) 0))
  (`PrimitiveComponent.SetMaterial` _mesh_2 0 "/Game/ArtPrototyping/Characters/DynamicDamage/M_Unwrapper.M_Unwrapper")
  (`MeshComponent.SetVectorParameterValueOnMaterials` _mesh_2 "CaptureLocation" (`self.K2_GetComponentLocation` _mesh_2))
  (`MeshComponent.SetVectorParameterValueOnMaterials` _mesh "HitLocation" Location)
  (`MeshComponent.SetScalarParameterValueOnMaterials` _mesh "DrawRadius" Radius)
  (`SceneCaptureComponent2D.CaptureScene` (`self.SceneCapture`))
  (`PrimitiveComponent.SetMaterial` (`self.Mesh`) 0 (`self.OldMat`)))