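; BP_Character is an AI-controlled character that takes damage and ragdolls on death.
; On begin play it caches its controller as an AI_Character, and it forwards incoming damage to its health component.
; The health component's death event disables the AI controller, zeroes walk speed, turns off capsule collision and triggers ragdoll through the physical animation component.
; A helper function returns current speed from velocity.
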(event `self.ReceiveBeginPlay`
  (bind _asai_character (cast `/Game/Characters/AI/AI_Character` (`self.GetController`)))
  (set `self.AIController` _asai_character))

(event `/Game/Player/Blueprints/BPI_Lifecycle.TakeDamage`
  (params (Amount :type Integer))
  (`/Game/Player/Blueprints/BPC_Health.TakeDamage` (`self.BPC_Health`) Amount))

(event `self.BPC_Health.OnDeath`
  (set `/Game/Characters/AI/AI_Character.Enabled` false (`self.AIController`))
  (set `CharacterMovementComponent.MaxWalkSpeed` 0.0 (`self.CharacterMovement`))
  (`PrimitiveComponent.SetCollisionEnabled` (`self.CapsuleComponent`) "NoCollision")
  (`/Game/Characters/Blueprints/BPC_PhysicalAnim.Ragdoll` (`self.BPC_PhysicalAnim`)))

(fn `GetCurrentMoveSpeed`
  (returns (Speed :type "Float (double-precision)"))
  (return (`KismetMathLibrary.VSize` (`self.GetVelocity`))))

(fn `UserConstructionScript`)