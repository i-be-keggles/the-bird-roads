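; BPC_Health is a health component that tracks damage and death for its owning actor.
; Health starts at MaxHealth on BeginPlay, and TakeDamage lowers it to a floor of zero, calling Die whenever it is at zero.
; Die fires the OnDeath dispatcher, prints a debug message and optionally destroys the owner.
; GetHealth always returns 0 rather than the current Health.
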(event `self.ReceiveBeginPlay`
  (set `self.Health` (`self.MaxHealth`)))

(event `Die`
  (`self.OnDeath`)
  (`KismetSystemLibrary.PrintString` "Died")
  (if (`self.DestroyActorOnDeath`)
    (`Actor.K2_DestroyActor` (`self.GetOwner`))))

(event `/Game/Characters/Blueprints/BPI_Lifecycle.TakeDamage`
  (params (Amount :type Integer) (Hit :type "HitResult Structure") (Instigator :type "Actor Object Reference"))
  (bind _output_get (set `self.Health` (`KismetMathLibrary.Max` (- (`self.Health`) Amount))))
  (if (<= _output_get 0)
    (`self.Die`)))

(fn `GetHealth`
  (returns (Health :type Integer))
  (return 0))