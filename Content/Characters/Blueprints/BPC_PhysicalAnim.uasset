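; Actor component that switches the owning BP_Character's mesh into physics simulation for ragdoll.
; On BeginPlay it adds a PhysicalAnimationComponent to the owner and caches the character's mesh.
; TogglePhysicalAnimation and Ragdoll are identical, both enabling simulation on the pelvis and all bodies below it, with no path back.
; The added PhysicalAnimationComponent is stored but never configured or used.
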(event `self.ReceiveBeginPlay`
  (bind _returnvalue (`|AddComponentByClass` (`self.GetOwner`) "/Script/Engine.PhysicalAnimationComponent"))
  (set `self.PhysicalAnimationComponent` _returnvalue)
  (bind _asbp_character (cast `/Game/Characters/BP_Character` (`self.GetOwner`)))
  (set `self.Mesh` (`Character.Mesh` _asbp_character)))

(event `TogglePhysicalAnimation`
  (`SkeletalMeshComponent.SetAllBodiesBelowSimulatePhysics` (`self.Mesh`) "pelvis" true true))

(event `Ragdoll`
  (`SkeletalMeshComponent.SetAllBodiesBelowSimulatePhysics` (`self.Mesh`) "pelvis" true true))