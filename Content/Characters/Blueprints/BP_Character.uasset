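; AI-controlled character with randomised modular appearance that starts moving to a random point unless its AI is disabled on startup.
; Construction randomises coat colour from DT_Coats through a dynamic material, picks hair and hat meshes, and links clothing to the body via leader pose.
; Damage feeds the health component, marks the instigator hostile on the AI controller and triggers physical-animation hit reactions.
; Death notifies the controller, stops movement, disables capsule collision and ragdolls.
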(event `self.ReceiveBeginPlay`
  (bind _asai_character (cast `/Game/Characters/AI/AI_Character` (`self.GetController`)))
  (bind _output_get (set `self.AIController` _asai_character))
  (if (not (`self.DisableAIOnStartup`))
    (`/Game/Characters/AI/AI_Character.GotoRandomPoint` _output_get)))

(event `/Game/Characters/Blueprints/BPI_Lifecycle.TakeDamage`
  (params (Amount :type Integer) (Hit :type "HitResult Structure") (Instigator :type "Actor Object Reference"))
  (`/Game/Characters/Blueprints/BPC_Health.TakeDamage` (`self.BPC_Health`) Amount Hit null)
  (`KismetArrayLibrary.Array_AddUnique` (`/Game/Characters/AI/AI_Character.HostileActors` (`self.AIController`)) Instigator)
  (`/Game/Characters/Blueprints/BPC_PhysicalAnim.HitReaction` (`self.BPC_PhysicalAnim`) Hit (`KismetMathLibrary.SelectFloat` 1.0 0.2 (> (`/Game/Characters/Blueprints/BPC_Health.Health` (`self.BPC_Health`)) 0)))
  (`self.OnTakeDamage`))

(event `self.BPC_Health.OnDeath`
  (`/Game/Characters/AI/AI_Character.OnDeath` (`self.AIController`))
  (set `CharacterMovementComponent.MaxWalkSpeed` 0.0 (`self.CharacterMovement`))
  (`PrimitiveComponent.SetCollisionEnabled` (`self.CapsuleComponent`) "NoCollision")
  (`/Game/Characters/Blueprints/BPC_PhysicalAnim.Ragdoll` (`self.BPC_PhysicalAnim`)))

(fn `GetCurrentMoveSpeed`
  (returns (Speed :type "Float (double-precision)"))
  (return (`KismetMathLibrary.VSize` (`self.GetVelocity`))))

(fn `GetHealth`
  (returns (Health :type Integer))
  (return (`/Game/Characters/Blueprints/BPC_Health.Health` (`self.BPC_Health`))))

(fn `UserConstructionScript`
  (bind _outrownames (`DataTableFunctionLibrary.GetDataTableRowNames` "/Game/ArtPrototyping/Characters/Clothing/DT_Coats.DT_Coats"))
  (bind _returnvalue (`|GetDataTableRow` "/Game/ArtPrototyping/Characters/Clothing/DT_Coats.DT_Coats" (`KismetArrayLibrary.Array_Random` _outrownames))
    (:`then`
      (bind _returnvalue_2 (`PrimitiveComponent.CreateDynamicMaterialInstance` (`self.Coat`) 0 "/Game/ArtPrototyping/Characters/M_Character.M_Character" "None"))
      (`MaterialInstanceDynamic.SetVectorParameterValue` _returnvalue_2 "CoatColour" (`KismetMathLibrary.Conv_ColorToLinearColor` (`KismetArrayLibrary.Array_Random` (`.Colours_6_FC937F4047E05E94DA84548F270F33AE` (break `/Game/ArtPrototyping/Characters/Clothing/S_ClothingItem` _returnvalue)))))
      (`SkeletalMeshComponent.SetSkeletalMeshAsset` (`self.Hair`) (`KismetArrayLibrary.Array_Random` (`|MakeArray` "/Game/ArtPrototyping/Characters/Clothing/Meshes/Mustache.Mustache" null null :!type "SkeletalMesh Object Reference")))
      (`SkeletalMeshComponent.SetSkeletalMeshAsset` (`self.Hat`) (`KismetArrayLibrary.Array_Random` (`|MakeArray` "/Game/ArtPrototyping/Characters/Clothing/Meshes/HatTest.HatTest" "/Game/ArtPrototyping/Characters/Clothing/Meshes/Cap.Cap" "/Game/ArtPrototyping/Characters/Clothing/Meshes/Goggles.Goggles" null :!type "SkeletalMesh Object Reference")))
      (`SkinnedMeshComponent.SetLeaderPoseComponent` (`self.Hat`) (`self.Mesh`) false false)
      (`SkinnedMeshComponent.SetLeaderPoseComponent` (`self.Shirt`) (`self.Mesh`) false false)
      (`SkinnedMeshComponent.SetLeaderPoseComponent` (`self.Pants`) (`self.Mesh`) false false)
      (`SkinnedMeshComponent.SetLeaderPoseComponent` (`self.Shoes`) (`self.Mesh`) false false)
      (`SkinnedMeshComponent.SetLeaderPoseComponent` (`self.Hair`) (`self.Mesh`) false false)
      (`SkinnedMeshComponent.SetLeaderPoseComponent` (`self.Coat`) (`self.Mesh`) false false))))