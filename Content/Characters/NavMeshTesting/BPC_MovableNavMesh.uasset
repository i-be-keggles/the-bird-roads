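; BPC_MovableNavMesh is a component that builds a static stand-in of its owner, apparently to provide navmesh for a movable actor.
; On BeginPlay it spawns BP_EmptyBakedNavmesh at the owner's XY and a random depth far below the origin.
; It copies visible-in-game, collision-enabled static meshes from the owner and its child actors onto that actor, preserving owner-relative transforms.
; It then spawns a BP_NavigationInvokerDummy at the copy's location.
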(event `self.ReceiveBeginPlay`
  (`self.SpawnStaticCopy`))

(fn `SpawnStaticCopy`
  (locals (Meshes :type "Array of StaticMeshComponent Object Reference"))
  (bind _returnvalue (`self.GetOwner`))
  (bind (_returnvalue_x _returnvalue_y) (`KismetMathLibrary.BreakVector` (`Actor.K2_GetActorLocation` _returnvalue)))
  (bind _returnvalue_2 (`|SpawnActorFromClass` "/Game/Characters/NavMeshTesting/BP_EmptyBakedNavmesh.BP_EmptyBakedNavmesh_C" (`KismetMathLibrary.MakeTransform` (`KismetMathLibrary.MakeVector` _returnvalue_x _returnvalue_y (`KismetMathLibrary.RandomFloatInRange` -30000.0 -50000.0))) "Undefined" "MultiplyWithRoot" null null))
  (set `self.StaticActorCopy` _returnvalue_2)
  (`|ExecutionSequence`
    (:`then_0`
      (for _array_element (`Actor.K2_GetComponentsByClass` _returnvalue "/Script/Engine.StaticMeshComponent")
        (if (and (`PrimitiveComponent.K2_IsCollisionEnabled` _array_element) (not (`SceneComponent.bHiddenInGame` _array_element)))
          (`KismetArrayLibrary.Array_Add` (`local.Meshes`) _array_element))))
    (:`then_1`
      (for _array_element_2 (`Actor.GetAllChildActors` _returnvalue true)
        (for _array_element_3 (`Actor.K2_GetComponentsByClass` _array_element_2 "/Script/Engine.StaticMeshComponent")
          (if (and (`PrimitiveComponent.K2_IsCollisionEnabled` _array_element_3) (not (`SceneComponent.bHiddenInGame` _array_element_3)))
            (`KismetArrayLibrary.Array_Add` (`local.Meshes`) _array_element_3)))))
    (:`then_2`
      (for _array_element_4 (`local.Meshes`)
        (bind _returnvalue_3 (`|AddComponentByClass` (`self.StaticActorCopy`) "/Script/Engine.StaticMeshComponent" false (`KismetMathLibrary.MakeRelativeTransform` (`SceneComponent.K2_GetComponentToWorld` _array_element_4) (`Actor.GetTransform` (`self.GetOwner`)))))
        (`StaticMeshComponent.SetStaticMesh` _returnvalue_3 (`StaticMeshComponent.StaticMesh` _array_element_4))))
    (:`then_3`
      (`|SpawnActorFromClass` "/Game/Characters/NavMeshTesting/BP_NavigationInvokerDummy.BP_NavigationInvokerDummy_C" (`KismetMathLibrary.MakeTransform` (`Actor.K2_GetActorLocation` (`self.StaticActorCopy`))) "Undefined" "MultiplyWithRoot" null null))))