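; Test character that chases a BP_DebugMesherFollow actor using navmesh paths computed in an offset space.
; Each tick it shifts start and target from Parent's frame to Movable's, finds a synchronous path, then maps points back, translation only.
; It draws debug boxes at path points and steers manually via movement input and control yaw, advancing PathIndex within 50 units.
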(event `self.ReceiveBeginPlay`
  (bind _returnvalue (`GameplayStatics.GetActorOfClass` "/Game/Characters/NavMeshTesting/BP_DebugMesherFollow.BP_DebugMesherFollow_C"))
  (set `self.Follow` _returnvalue)
  (`self.MoveTo` (`self.K2_GetActorLocation` (`self.Follow`)))
  (`self.MoveToNextPathPoint`))

(event `self.ReceiveTick`
  (params (DeltaSeconds :type "Float (single-precision)"))
  (`self.MoveTo` (`self.K2_GetActorLocation` (`self.Follow`)))
  (for _array_element (`NavigationPath.PathPoints` (`self.Path`))
    (bind _out (`self.ToWorld` _array_element))
    (`KismetSystemLibrary.DrawDebugBox` _out (10.0 10.0 10.0) (struct :`R` 0.539541 :`G` 0.71108 :`B` 1.0 :`A` 1.0))
    (`self.MoveToNextPathPoint`)))

(event `MoveToNextPathPoint`
  (bind _out (`self.ToWorld` (`|GetArrayItem` (`NavigationPath.PathPoints` (`self.Path`)) (`self.PathIndex`))))
  (`|ExecutionSequence`
    (:`then_0`
      (bind _returnvalue (- _out (`self.K2_GetActorLocation`)))
      (bind _returnvalue_2 (`KismetMathLibrary.VSize` _returnvalue))
      (if (< _returnvalue_2 50.0)
        (bind _result (`/Engine/EditorBlueprintResources/StandardMacros.IncrementInt` (`self.PathIndex`))
          (:`  `
            (if (>= _result (`KismetArrayLibrary.Array_Length` (`NavigationPath.PathPoints` (`self.Path`))))
              (`/Engine/EditorBlueprintResources/StandardMacros.DecrementInt` (`self.PathIndex`)))))))
    (:`then_1`
      (`PawnMovementComponent.AddInputVector` (`self.CharacterMovement`) (* (/ _returnvalue _returnvalue_2) 1.0) false)
      (bind (_returnvalue_roll _returnvalue_pitch _returnvalue_yaw) (`KismetMathLibrary.BreakRotator` (`KismetMathLibrary.Conv_VectorToRotator` _returnvalue)))
      (`Controller.SetControlRotation` (`self.GetController`) (`KismetMathLibrary.MakeRotator` 0.0 0.0 _returnvalue_yaw)))))

(event `MoveTo`
  (params (Position :type "Vector Structure"))
  (bind _returnvalue (`NavigationSystemV1.FindPathToLocationSynchronously` (+ (- (`self.K2_GetActorLocation`) (`self.K2_GetActorLocation` (`self.Parent`))) (`self.K2_GetActorLocation` (`self.Movable`))) (+ (- Position (`self.K2_GetActorLocation` (`self.Parent`))) (`self.K2_GetActorLocation` (`self.Movable`))) (`AIBlueprintHelperLibrary.GetAIController` null) null))
  (set `self.Path` _returnvalue))

(fn `ToWorld`
  (params (In :type "Vector Structure"))
  (returns (Out :type "Vector Structure"))
  (return (+ (- In (`self.K2_GetActorLocation` (`self.Movable`))) (`self.K2_GetActorLocation` (`self.Parent`)))))

(fn `UserConstructionScript`)