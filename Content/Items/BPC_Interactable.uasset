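; Interactable component that gives its owner an interact event and an on-screen prompt.
; Interact relays the call to listeners through the OnInteract dispatcher.
; Observe builds the prompt by querying Enhanced Input for the first key mapped to IA_Interact and prefixing its bracketed display name to PromptText.
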(event `/Game/Items/BPI_Interactable.Interact`
  (`self.OnInteract`))

(fn `Observe`
  (returns (Prompt :type String))
  (return (`KismetStringLibrary.Concat_StrStr` "[" (`KismetTextLibrary.Conv_TextToString` (`KismetInputLibrary.Key_GetDisplayName` (`|GetArrayItem` (`EnhancedInputSubsystemInterface.QueryKeysMappedToAction` (pcsubsystem `EnhancedInputLocalPlayerSubsystem` (`GameplayStatics.GetPlayerController` 0)) "/Game/Player/Input/Actions/IA_Interact.IA_Interact")))) "] " (`self.Prompt Text`))))