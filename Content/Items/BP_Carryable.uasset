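; BP_Carryable is a physics item the player can pick up, carry, drop and place on cargo grids.
; A held interaction finds a nearby BP_Player, attaches the mesh to its capsule if it carries nothing, and removes the item from any grid.
; Drop restores physics and collision and notifies listeners.
; Cargo items then trace downward to request a slot on the BP_CargoGrid beneath.
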(event `self.ReceiveBeginPlay`
  (bind _asbp_player (cast `/Game/Player/Blueprints/BP_Player` (`Controller.K2_GetPawn` (`GameplayStatics.GetPlayerController` 0))))
  (set `self.Player` _asbp_player))

(event `self.BPC_Interactable.OnInteract`
  (params (Held :type Boolean))
  (bind _cargogrid (`self.CargoGrid`))
  (bind _staticmesh (`self.StaticMesh`))
  (if Held
    (bind _outactors (`KismetSystemLibrary.SphereOverlapActors` (`SceneComponent.K2_GetComponentLocation` (`self.StaticMesh`)) 500.0 (`|MakeArray` "ObjectTypeQuery3" :!type "EObjectTypeQuery Enum") "/Game/Player/Blueprints/BP_Player.BP_Player_C"))
    (if (> (`KismetArrayLibrary.Array_Length` _outactors) 0)
      (bind _asbp_player (cast `/Game/Player/Blueprints/BP_Player` (`|GetArrayItem` _outactors))
        (:`then`
          (bind _output_get (set `self.Player` _asbp_player))
          (`/Engine/EditorBlueprintResources/StandardMacros.IsValid` (`/Game/Player/Blueprints/BP_Player.CarryingObject` _output_get)
            (:`Is Not Valid`
              (`/Game/Player/Blueprints/BP_Player.StartCarrying` _output_get)
              (`PrimitiveComponent.SetSimulatePhysics` _staticmesh false)
              (`PrimitiveComponent.SetCollisionEnabled` _staticmesh "NoCollision")
              (set `/Game/Player/Blueprints/BP_Player.CarryingObject` self _asbp_player)
              (`SceneComponent.K2_AttachToComponent` (`self.StaticMesh`) (`Character.CapsuleComponent` _asbp_player) "None" "SnapToTarget" "SnapToTarget" "SnapToTarget" true)
              (`SceneComponent.K2_SetRelativeTransform` (`self.StaticMesh`) (`KismetMathLibrary.MakeTransform` (50.0 0.0 -20.0)) false true)
              (`/Engine/EditorBlueprintResources/StandardMacros.IsValid` _cargogrid
                (:`Is Valid`
                  (`/Game/Ships/Blueprints/BP_CargoGrid.RemoveItem` _cargogrid self)
                  (set `self.CargoGrid` null))))))
        (:`CastFailed`
          (`KismetSystemLibrary.PrintString` "Carryable cast failed")))
      (else
        (`KismetSystemLibrary.PrintString` "No player in range of carryable")))))

(event `Drop`
  (bind _player (`self.Player`))
  (bind _staticmesh (`self.StaticMesh`))
  (bind _staticmesh_2 (`self.StaticMesh`))
  (`|ExecutionSequence`
    (:`then_0`
      (`SceneComponent.K2_SetRelativeLocation` _staticmesh_2 (100.0 0.0 -20.0) false false)
      (`SceneComponent.K2_DetachFromComponent` _staticmesh_2 "KeepWorld" "KeepWorld" "KeepWorld" true)
      (`PrimitiveComponent.SetSimulatePhysics` _staticmesh true)
      (`PrimitiveComponent.SetCollisionEnabled` _staticmesh "QueryAndPhysics")
      (set `/Game/Player/Blueprints/BP_Player.CarryingObject` null _player)
      (`/Game/Player/Blueprints/BP_Player.StopCarrying` _player)
      (`self.OnDropped`))
    (:`then_1`
      (if (`self.CargoGridItem`)
        (`self.TryPlaceCargoItem`)))))

(event `TryPlaceCargoItem`
  (bind _returnvalue (`SceneComponent.K2_GetComponentLocation` (`self.StaticMesh`)))
  (bind (_outhit _returnvalue_2) (`KismetSystemLibrary.LineTraceSingle` _returnvalue (- _returnvalue (0.0 0.0 200.0)) "TraceTypeQuery1"))
  (if _returnvalue_2
    (bind (_bblockinghit _binitialoverlap _time _distance _location _impactpoint _normal _impactnormal _physmat _hitactor) (`GameplayStatics.BreakHitResult` _outhit))
    (bind _asbp_cargo_grid (cast `/Game/Ships/Blueprints/BP_CargoGrid` _hitactor))
    (bind (_x _y) (`/Game/Ships/Blueprints/BP_CargoGrid.GetSlotFromWorldPos` _asbp_cargo_grid _impactpoint))
    (`/Game/Ships/Blueprints/BP_CargoGrid.TryAddItem` _asbp_cargo_grid self _x _y)))

(fn `UserConstructionScript`
  (`parent.UserConstructionScript`))