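; BP_RepairCrate is an interactable crate that restocks the repair kits in the player's equipment.
; When its BPC_Interactable component reports a non-held interaction, it loops through the equipment and sets each BP_RepairKit's current ammo to its maximum.
; A kit that is active also updates the ammo display on its HUD.
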(event `self.BPC_Interactable.OnInteract`
  (params (Held :type Boolean))
  (if (not Held)
    (for _array_element (`/Game/Player/Blueprints/BP_Player.Equipment` (`self.Player`))
      (bind _asbp_repair_kit (cast `/Game/Player/Equipment/BP_RepairKit` _array_element))
      (bind _output_get (set `/Game/Player/Equipment/BP_RepairKit.CurAmmo` (`/Game/Player/Equipment/BP_RepairKit.MaxAmmo` _asbp_repair_kit) _asbp_repair_kit))
      (if (`/Game/Player/Equipment/BP_Equipment.Active` _asbp_repair_kit)
        (`/Game/UI/Widgets/WB_FirstPersonHUD.UpdateAmmo` (`/Game/Player/Equipment/BP_Equipment.HUD` _asbp_repair_kit) _output_get)))))

(fn `UserConstructionScript`
  (`parent.UserConstructionScript`))