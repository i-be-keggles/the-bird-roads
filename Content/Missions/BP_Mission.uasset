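; BP_Mission represents a mission made of an ordered list of objectives that are completed one after another.
; On BeginPlay it binds to the current objective's completion events and gets the mission HUD from the first-person game mode's MissionManager.
; Each completed objective moves the bindings to the next one, and the last fires OnComplete.
; Objective and sub-objective completions refresh the HUD, while GenerateMission is an empty stub.
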(event `self.ReceiveBeginPlay`
  (`self.Initialise`))

(event `Initialise`
  (if (`KismetArrayLibrary.Array_IsNotEmpty` (`self.Objectives`))
    (bind _objective (`self.GetCurrentObjective`))
    (add `/Game/Missions/BP_MissionObjective.OnCompleted` _objective (delegate `CompletedObjective`))
    (add `/Game/Missions/BP_MissionObjective.OnSubObjectiveCompleted` _objective (delegate `CompleteSubObjective`))
    (bind _asbp_first_person_game_mode (cast `/Game/Player/Blueprints/BP_FirstPersonGameMode` (`GameplayStatics.GetGameMode`)))
    (bind _output_get (set `self.MissionManager` (`/Game/Player/Blueprints/BP_FirstPersonGameMode.MissionManager` _asbp_first_person_game_mode)))
    (set `self.Mission HUD` (`/Game/Missions/BP_MissionManager.MissionHUD` _output_get))))

(event `CompletedObjective`
  (`KismetSystemLibrary.PrintString` "YAY COMPLETED OBJECTIVE!!")
  (if (== (`self.ObjectiveID`) (`KismetArrayLibrary.Array_LastIndex` (`self.Objectives`)))
    (`self.CompleteMission`)
    (else
      (bind _objective (`self.GetCurrentObjective`))
      (remove `/Game/Missions/BP_MissionObjective.OnCompleted` _objective (delegate `CompletedObjective`))
      (remove `/Game/Missions/BP_MissionObjective.OnSubObjectiveCompleted` _objective (delegate `CompleteSubObjective`))
      (`/Engine/EditorBlueprintResources/StandardMacros.IncrementInt` (`self.ObjectiveID`)
        (:`  `
          (bind _objective_2 (`self.GetCurrentObjective`))
          (add `/Game/Missions/BP_MissionObjective.OnCompleted` _objective_2 (delegate `CompletedObjective`))
          (add `/Game/Missions/BP_MissionObjective.OnSubObjectiveCompleted` _objective_2 (delegate `CompleteSubObjective`))
          (`/Game/UI/Widgets/WBP_MissionHUD.UpdateMission` (`self.Mission HUD`) self))))))

(event `CompleteSubObjective`
  (`/Game/UI/Widgets/WBP_MissionHUD.UpdateMission` (`self.Mission HUD`) self))

(event `CompleteMission`
  (`/Game/UI/Widgets/WBP_MissionHUD.UpdateMission` (`self.Mission HUD`) self)
  (`self.OnComplete`))

(fn `Generate Mission`)

(fn `GetCurrentObjective`
  (returns (Objective :type "/Game/Missions/BP_MissionObjective Object Reference"))
  (return (`|GetArrayItem` (`self.Objectives`) (`self.ObjectiveID`))))

(fn `UserConstructionScript`)