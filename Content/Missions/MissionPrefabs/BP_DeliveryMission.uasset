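; Mission prefab that generates a cargo delivery job from its mission giver to another randomly chosen giver.
; GenerateMission shuffles the manager's givers, takes the first other one with a valid delivery location, and titles the mission after it.
; It spawns one or two carryable crates, each with a delivery objective targeting that location, grouped under a multi-objective.
; Objective actors attach to the mission, and the multi-objective initialises before the mission.
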(fn `Generate Mission`
  (locals (DeliveryLocation :type "Actor Object Reference") (MultiObjective :type "/Game/Missions/Objectives/BP_MultiObjective Object Reference") (MissionGivers :type "Array of /Game/Missions/BP_MissionGiver Object Reference"))
  (bind (_returnvalue_location _returnvalue_rotation _returnvalue_scale) (`KismetMathLibrary.BreakTransform` (`self.GetTransform`)))
  (bind _output_get (set `local.MissionGivers` (`/Game/Missions/BP_MissionManager.MissionGivers` (`self.MissionManager`))))
  (`KismetArrayLibrary.Array_RemoveItem` _output_get (`self.MissionGiver`))
  (`KismetArrayLibrary.Array_Shuffle` (`local.MissionGivers`))
  (for _array_element (`local.MissionGivers`)
    (if (and (!= _array_element (`self.MissionGiver`)) (`KismetSystemLibrary.IsValid` (`/Game/Missions/BP_MissionGiver.DeliveryLocation` _array_element)))
      (set `local.DeliveryLocation` (`/Game/Missions/BP_MissionGiver.DeliveryLocation` _array_element))
      (set `self.Title` (`KismetStringLibrary.Conv_StringToName` (`KismetStringLibrary.Concat_StrStr` "Deliver cargo to " (`KismetStringLibrary.Conv_NameToString` (`/Game/Missions/BP_MissionGiver.Name` _array_element)))))
      (`|ExecutionSequence`
        (:`then_0`
          ;[1 1 1] Set up multi objective
          (bind _returnvalue (`|SpawnActorFromClass` "/Game/Missions/Objectives/BP_MultiObjective.BP_MultiObjective_C" (`self.GetTransform`) "Undefined" "MultiplyWithRoot" null null))
          (bind _output_get_2 (set `local.MultiObjective` _returnvalue))
          (`KismetArrayLibrary.Array_Add` (`self.Objectives`) _output_get_2)
          (`self.K2_AttachToActor` _output_get_2 self "None" "SnapToTarget" "SnapToTarget" "KeepWorld" true))
        (:`then_1`
          (for _index (range 1 (+ (`KismetMathLibrary.RandomIntegerInRange` 1 2) 1))
            (bind _returnvalue_2 (`|SpawnActorFromClass` "/Game/Items/BP_Carryable.BP_Carryable_C" (`KismetMathLibrary.MakeTransform` (+ _returnvalue_location (* (`self.GetActorRightVector`) (`KismetMathLibrary.Conv_DoubleToVector` 100.0)) (0.0 0.0 100.0)) _returnvalue_rotation _returnvalue_scale) "AdjustIfPossibleButAlwaysSpawn" "MultiplyWithRoot" null null))
            (bind _returnvalue_3 (`|SpawnActorFromClass` "/Game/Missions/Objectives/BP_DeliveryObjective.BP_DeliveryObjective_C" (`self.GetTransform`) "Undefined" "MultiplyWithRoot" null null))
            (set `/Game/Missions/BP_MissionObjective.Description` (`KismetTextLibrary.Conv_StringToText` (`KismetStringLibrary.Concat_StrStr` "Deliver crate " (`KismetStringLibrary.Conv_IntToString` _index))) _returnvalue_3)
            (set `/Game/Missions/Objectives/BP_DeliveryObjective.DeliveryItem` _returnvalue_2 _returnvalue_3)
            (`KismetArrayLibrary.Array_Add` (`/Game/Missions/Objectives/BP_MultiObjective.Objectives` (`local.MultiObjective`)) _returnvalue_3)
            (set `/Game/Missions/Objectives/BP_DeliveryObjective.DeliveryLocation` (`local.DeliveryLocation`) _returnvalue_3)
            (`/Game/Missions/BP_MissionObjective.Initialise` _returnvalue_3)
            (`self.K2_AttachToActor` _returnvalue_3 self "None" "SnapToTarget" "SnapToTarget" "KeepWorld" true))
          ;[1 1 1] Initialise multiobjective
          (`/Game/Missions/BP_MissionObjective.Initialise` (`local.MultiObjective`)))
        (:`then_2`
          ;[1 1 1] Initialise Mission
          (`self.Initialise`)
          (return))))))

(fn `UserConstructionScript`
  (`parent.UserConstructionScript`))