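; Mission prefab that generates a ship combat mission to neutralise a target airship.
; GenerateMission uses the game mode's ShipManager to spawn a random blimp or medium airship with crew in a box above the mission giver.
; It attaches a BP_ShipCombatObjective targeting that ship, then initialises the objective and mission.
; An unreachable branch holds cargo-delivery generation logic using a multi-objective.
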(fn `Generate Mission`
  (locals (DeliveryLocation :type "Actor Object Reference") (MultiObjective :type "/Game/Missions/Objectives/BP_MultiObjective Object Reference") (MissionGivers :type "Array of /Game/Missions/BP_MissionGiver Object Reference"))
  (bind _asbp_first_person_game_mode (cast `/Game/Player/Blueprints/BP_FirstPersonGameMode` (`GameplayStatics.GetGameMode`)))
  (bind _shipmanager (`/Game/Player/Blueprints/BP_FirstPersonGameMode.ShipManager` _asbp_first_person_game_mode))
  (bind _spawnedairship (`/Game/Ships/Blueprints/BP_ShipSwitchPrototype.SpawnAirship` :`self` _shipmanager :`Airship Class` (`KismetArrayLibrary.Array_Random` (`|MakeArray` "/Game/Ships/Prefabs/BP_Airship_Blimp.BP_Airship_Blimp_C" "/Game/Ships/Prefabs/BP_Airship_Medium.BP_Airship_Medium_C" :!type "/Game/Ships/Blueprints/BP_Airship Class Reference")) :`FactionID` 5 :`Location` (`KismetMathLibrary.RandomPointInBoundingBox` (+ (`self.K2_GetActorLocation` (`self.MissionGiver`)) (0.0 0.0 2000.0)) (5000.0 5000.0 500.0))))
  (`/Game/Ships/Blueprints/BP_ShipSwitchPrototype.SpawnAirshipCrew` _shipmanager _spawnedairship)
  (bind _returnvalue (`|SpawnActorFromClass` "/Game/Missions/Objectives/BP_ShipCombatObjective.BP_ShipCombatObjective_C" (`self.GetTransform`) "Undefined" "MultiplyWithRoot" null null))
  (`self.K2_AttachToActor` _returnvalue self "None" "KeepWorld" "SnapToTarget" "KeepWorld" true)
  (set `/Game/Missions/Objectives/BP_ShipCombatObjective.TargetShip` _spawnedairship _returnvalue)
  (set `/Game/Missions/BP_MissionObjective.Description` "Neutralise target airship" _returnvalue)
  (`KismetArrayLibrary.Array_Add` (`self.Objectives`) _returnvalue)
  (`/Game/Missions/BP_MissionObjective.Initialise` _returnvalue)
  (`self.Initialise`))

(fn `UserConstructionScript`
  (`parent.UserConstructionScript`))