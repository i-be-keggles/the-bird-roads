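; BP_DeliveryObjective is a mission objective that completes when a designated item is delivered to a location.
; On BeginPlay it binds to the begin overlap event of the DeliveryLocation actor.
; When the overlapping actor is DeliveryItem, it prints a "Delivered" message and calls Complete.
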(event `self.ReceiveBeginPlay`
  (`parent.ReceiveBeginPlay`)
  (add `Actor.OnActorBeginOverlap` (`self.DeliveryLocation`) (delegate `OnActorBeginOverlap_Event`)))

(event `OnActorBeginOverlap_Event`
  (params (OverlappedActor :type "Actor Object Reference") (OtherActor :type "Actor Object Reference"))
  (if (== OtherActor (`self.DeliveryItem`))
    (`KismetSystemLibrary.PrintString` "Delivered")
    (`self.Complete`)))

(fn `UserConstructionScript`
  (`parent.UserConstructionScript`))