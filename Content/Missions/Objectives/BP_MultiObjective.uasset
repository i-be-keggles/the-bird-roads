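; BP_MultiObjective is a composite mission objective that completes when all objectives in its Objectives array are completed.
; On BeginPlay it binds CheckCompleted to each child objective's OnCompleted event.
; Each child completion fires the OnSubObjectiveCompleted dispatcher, then IsCompleted checks every child's Completed flag and calls Complete on the parent objective once all are true.
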(event `self.ReceiveBeginPlay`
  (`parent.ReceiveBeginPlay`)
  (for _array_element (`self.Objectives`)
    (add `self.OnCompleted` _array_element (delegate `CheckCompleted`))))

(event `CheckCompleted`
  (`self.OnSubObjectiveCompleted`)
  (bind _completed (`self.IsCompleted`))
  (if _completed
    (`self.Complete`)))

(fn `IsCompleted`
  (returns (Completed :type Boolean))
  (locals (Complete :type Boolean :default true))
  (set `local.Complete` true)
  (for _array_element (`self.Objectives`)
    (if (not (`/Game/Missions/BP_MissionObjective.Completed` _array_element))
      (set `local.Complete` false)))
  (return (`local.Complete`)))

(fn `UserConstructionScript`
  (`parent.UserConstructionScript`))