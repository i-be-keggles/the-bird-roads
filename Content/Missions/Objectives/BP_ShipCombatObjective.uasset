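; BP_ShipCombatObjective is a mission objective to neutralise a target airship by knocking out all its cannons and propellors.
; On initialise it records the ship's active cannon and propellor counts, binds to the ship's hit event and runs a first completion check.
; Each check recounts active components, completing the objective when both reach zero, or otherwise rewriting the progress description and refreshing the mission HUD.
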(event `self.ReceiveBeginPlay`
  (`parent.ReceiveBeginPlay`))

(event `self.Initialise`
  (bind _targetship (`self.TargetShip`))
  (`parent.Initialise`)
  (`/Engine/EditorBlueprintResources/StandardMacros.IsValid` _targetship
    (:`Is Valid`
      (bind _count (`/Game/Ships/Blueprints/BP_Airship.GetActiveComponentCount` _targetship "/Game/Ships/Components/BP_ShipComponent_Cannon.BP_ShipComponent_Cannon_C"))
      (set `self.Cannons` _count)
      (bind _count_2 (`/Game/Ships/Blueprints/BP_Airship.GetActiveComponentCount` _targetship "/Game/Ships/Components/BP_ShipComponent_Propellor.BP_ShipComponent_Propellor_C"))
      (set `self.Propellors` _count_2)
      (add `/Game/Ships/Blueprints/BP_Airship.OnHit` (`self.TargetShip`) (delegate `CheckComplete`))
      (`self.CheckComplete`))))

(event `CheckComplete`
  (bind _targetship (`self.TargetShip`))
  (bind _mission_manager (`self.Mission Manager`))
  (bind _cannons (`self.Cannons`))
  (bind _propellors (`self.Propellors`))
  (`/Engine/EditorBlueprintResources/StandardMacros.IsValid` _targetship
    (:`Is Valid`
      (bind _count (`/Game/Ships/Blueprints/BP_Airship.GetActiveComponentCount` _targetship "/Game/Ships/Components/BP_ShipComponent_Cannon.BP_ShipComponent_Cannon_C"))
      (bind _count_2 (`/Game/Ships/Blueprints/BP_Airship.GetActiveComponentCount` _targetship "/Game/Ships/Components/BP_ShipComponent_Propellor.BP_ShipComponent_Propellor_C"))
      (if (and (<= _count_2 0) (<= _count 0))
        (`KismetSystemLibrary.PrintString` "Ship neutralised")
        (`self.Complete`)
        (else
          (`KismetSystemLibrary.PrintString` "Ship not neutralised")
          (set `self.Description` (`KismetTextLibrary.Conv_StringToText` (`KismetStringLibrary.Concat_StrStr` "Neutralise target airship" (`KismetStringLibrary.Concat_StrStr` " \n" (`KismetStringLibrary.Conv_IntToString` (- _cannons _count)) "/" (`KismetStringLibrary.Conv_IntToString` _cannons) " cannons") (`KismetStringLibrary.Concat_StrStr` " \n" (`KismetStringLibrary.Conv_IntToString` (- _propellors _count_2)) "/" (`KismetStringLibrary.Conv_IntToString` _propellors) " propellors"))))
          (`/Game/UI/Widgets/WBP_MissionHUD.UpdateMission` (`/Game/Missions/BP_MissionManager.MissionHUD` _mission_manager) (`/Game/Missions/BP_MissionManager.ActiveMission` _mission_manager)))))))

(fn `UserConstructionScript`
  (`parent.UserConstructionScript`))