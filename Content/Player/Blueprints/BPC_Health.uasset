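; BPC_Health is a player health component that tracks Health against MaxHealth and removes its owner when health runs out.
; Health fills to MaxHealth on BeginPlay, and the TakeDamage event subtracts the given amount, clamped at zero.
; At zero it calls Die, which destroys the owning actor outright.
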(event `self.ReceiveBeginPlay`
  (set `self.Health` (`self.MaxHealth`)))

(event `Die`
  (`Actor.K2_DestroyActor` (`self.GetOwner`)))

(event `/Game/Player/Blueprints/BPI_Lifecycle.TakeDamage`
  (params (Amount :type Integer))
  (bind _output_get (set `self.Health` (`KismetMathLibrary.Max` (- (`self.Health`) Amount))))
  (if (<= _output_get 0)
    (`self.Die`)))