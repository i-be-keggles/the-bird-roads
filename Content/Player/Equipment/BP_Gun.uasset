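; BP_Gun is a player equipment Blueprint for a gun that shoots and reloads while active.
; It delegates gun logic to its BPCGun component, which receives the player's first-person camera on BeginPlay.
; Enhanced Input attack and reload actions call the component.
; The HUD ammo count refreshes after each shot and through the component's OnReloaded event.
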(event Custom|UpdateHud
  (Default|UpdateAmmo (Variables|Default|GetHUD) (Variables|/Game/Player/Weapons/BPC_Gun.BPC_Gun_C|GetCurAmmo (Variables|Default|GetBPC_Gun))))

(event Input|EnhancedActionEvents|EnhancedInputActionIA_Attack
  (params (ActionValue :type Boolean) (ElapsedSeconds :type Float%20%28double-precision%29) (TriggeredSeconds :type Float%20%28double-precision%29) (InputAction :type Input%20Action%20Object%20Reference :default "/Game/Player/Input/Actions/IA_Attack.IA_Attack"))
  (if (and ActionValue (Variables|Default|GetActive))
    (Default|Shoot (Variables|Default|GetBPC_Gun))
    (CallFunction|UpdateHud)))

(event Input|EnhancedActionEvents|EnhancedInputActionIA_Reload
  (params (ActionValue :type Boolean) (ElapsedSeconds :type Float%20%28double-precision%29) (TriggeredSeconds :type Float%20%28double-precision%29) (InputAction :type Input%20Action%20Object%20Reference :default "/Game/Player/Input/Actions/IA_Reload.IA_Reload"))
  (if (and ActionValue (Variables|Default|GetActive))
    (Default|Reload (Variables|Default|GetBPC_Gun))))

(event EventBeginPlay
  (|CallParentFunction)
  (EventDispatchers|BindEventtoOnReloaded (Variables|Default|GetBPC_Gun) (delegate Custom|UpdateHud))
  (Variables|/Game/Player/Weapons/BPC_Gun.BPC_Gun_C|SetCamera (Variables|Default|GetBPC_Gun) (Variables|/Game/Player/Blueprints/BP_Player.BP_Player_C|GetFirstPersonCamera (Variables|Default|GetPlayer))))

(fn ConstructionScript
  (|CallParentFunction))