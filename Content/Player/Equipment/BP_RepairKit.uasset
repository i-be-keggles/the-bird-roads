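; BP_RepairKit is player equipment that patches gas leaks and repairs ship components, using limited repair material as ammo.
; While active, attack runs a small sphere overlap at the player's trace impact point within interact range.
; The first gas leak found is removed, otherwise damaged non-gasbag components receive RepairMessage.
; Each successful use spawns a Niagara hit effect, consumes ammo and updates the HUD, which also reports repair status.
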(event `self.ReceiveBeginPlay`
  (`parent.ReceiveBeginPlay`)
  (set `self.CurAmmo` (`self.MaxAmmo`)))

(event `self.SetActive`
  (`parent.SetActive`)
  (`/Engine/EditorBlueprintResources/StandardMacros.IsValid` (`self.HUD`)
    (:`Is Valid`
      _)
    (:`Is Not Valid`
      (`KismetSystemLibrary.Delay` 0.2)))
  (`/Game/UI/Widgets/WB_FirstPersonHUD.UpdateAmmo` (`self.HUD`) (`self.CurAmmo`)))

(event `EnhancedInput|/Game/Player/Input/Actions/IA_Attack`
  (params (ActionValue :type Boolean) (ElapsedSeconds :type "Float (double-precision)") (TriggeredSeconds :type "Float (double-precision)") (InputAction :type "InputAction Object Reference" :default "/Game/Player/Input/Actions/IA_Attack.IA_Attack"))
  (bind _player (`self.Player`))
  (bind (_general_trace_bblockinghit _general_trace_binitialoverlap _general_trace_time _general_trace_distance _general_trace_location _general_trace_impactpoint _general_trace_normal _general_trace_impactnormal _general_trace_physmat _general_trace_hitactor) (`GameplayStatics.BreakHitResult` (`/Game/Player/Blueprints/BP_Player.General Trace` _player)))
  (:`Triggered`
    (if (and ActionValue (`self.Active`))
      (if (> (`self.CurAmmo`) 0)
        (`/Engine/EditorBlueprintResources/StandardMacros.IsValid` _general_trace_hitactor
          (:`Is Valid`
            (if (<= _general_trace_distance (`/Game/Player/Blueprints/BP_Player.InteractDistance` _player))
              (bind _outcomponents (`KismetSystemLibrary.SphereOverlapComponents` _general_trace_impactpoint 10.0 (`|MakeArray` "ObjectTypeQuery8" :!type "EObjectTypeQuery Enum")))
              (for _array_element _outcomponents
                (bind _asbpc_gas_leak (cast `/Game/Ships/Blueprints/BPC_GasLeak` (`SceneComponent.GetAttachParent` _array_element))
                  (:`then`
                    (`/Game/Ships/Blueprints/BPC_GasLeak.RemoveLeak` _asbpc_gas_leak)
                    (`NiagaraFunctionLibrary.SpawnSystemAtLocation` "/Game/FX/NiagaraSystems/NS_RepairHit.NS_RepairHit" _general_trace_impactpoint :!label _label)
                    (`/Engine/EditorBlueprintResources/StandardMacros.DecrementInt` (`self.CurAmmo`)
                      (:`  `
                        (`/Game/UI/Widgets/WB_FirstPersonHUD.UpdateAmmo` (`self.HUD`) (`self.CurAmmo`))
                        (break))))
                  (:`CastFailed`
                    (bind _asbp_ship_component (cast `/Game/Ships/Components/BP_ShipComponent` (`ActorComponent.GetOwner` _array_element)))
                    (if (!= (`GameplayStatics.GetObjectClass` _asbp_ship_component) "/Game/Ships/Components/BP_ShipComponent_Gasbag.BP_ShipComponent_Gasbag_C")
                      (if (< (`/Game/Ships/Components/BP_ShipComponent.Health` _asbp_ship_component) (`/Game/Ships/Components/BP_ShipComponent.MaxHealth` _asbp_ship_component))
                        (message `/Game/Ships/Components/BPI_ShipComponent.Repair` _asbp_ship_component (`self.RepairAmount`))
                        (`|ExecutionSequence`
                          (:`then_0`
                            (goto _label))
                          (:`then_1`
                            (if (not (< (`/Game/Ships/Components/BP_ShipComponent.Health` _asbp_ship_component) (`/Game/Ships/Components/BP_ShipComponent.MaxHealth` _asbp_ship_component)))
                              (`/Game/UI/Widgets/WB_FirstPersonHUD.DisplayMessage` (`self.HUD`) "Fully repaired" 1.5))))
                        (else
                          (`/Game/UI/Widgets/WB_FirstPersonHUD.DisplayMessage` (`self.HUD`) "Repair unneeded" 1.0))))))))))
        (else
          (`/Game/UI/Widgets/WB_FirstPersonHUD.DisplayMessage` (`self.HUD`) "No repair material" 1.0))))))

(fn `UserConstructionScript`
  (`parent.UserConstructionScript`))