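; Player weapon component that fires hitscan shots with a magazine, fire-rate limit and timed reload.
; Shoot traces forward from the component itself, spawning muzzle and reflected impact effects, sending damage and pushing physics objects unless their health component opts out.
; An empty magazine auto-reloads, then broadcasts OnReloaded.
; Tick animates procedurally: recoil kicks ease back to rest, while reloading pulls the gun back and spins it.
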(event `self.ReceiveBeginPlay`
  (set `self.CurAmmo` (`self.MagazineSize`))
  (set `self.InitialLocation` (`self.RelativeLocation`))
  (set `self.Camera` self))

(event `self.ReceiveTick`
  (params (DeltaSeconds :type "Float (single-precision)"))
  (bind _reloading (`self.Reloading`))
  (bind (_relativerotation_roll _relativerotation_pitch _relativerotation_yaw) (`KismetMathLibrary.BreakRotator` (`self.RelativeRotation`)))
  (bind _output_get (set `self.RecoilPos` (`KismetMathLibrary.VLerp` (`self.RecoilPos`) (0.0 0.0 0.0) (* DeltaSeconds 5.0))))
  (`self.K2_SetRelativeLocation` (+ _output_get (`self.InitialLocation`)))
  (`self.K2_SetRelativeRotation` (`KismetMathLibrary.SelectRotator` (`KismetMathLibrary.MakeRotator` 90.0 0.0 (+ _relativerotation_yaw (* DeltaSeconds 1500.0))) (struct) _reloading))
  (if _reloading
    (set `self.RecoilPos` (-50.0 0.0 0.0))))

(event `Reload`
  (if (not (or (`self.Reloading`) (== (`self.CurAmmo`) (`self.MagazineSize`))))
    (set `self.Reloading` true)
    (set `self.CanShoot` false)
    (`KismetSystemLibrary.Delay` (`self.ReloadTime`))
    (set `self.CurAmmo` (`self.MagazineSize`))
    (set `self.CanShoot` true)
    (set `self.Reloading` false)
    (`self.OnReloaded`)))

(event `Shoot`
  (bind _returnvalue (`self.GetOwner`))
  (bind _returnvalue_2 (`self.GetOwner`))
  (bind _camera (`self.Camera`))
  (bind _curammo (`self.CurAmmo`))
  (bind _returnvalue_3 (`self.K2_GetComponentLocation` _camera))
  (if (and (`self.CanShoot`) (not (`self.Reloading`)))
    (`|ExecutionSequence`
      (:`then_0`
        (bind (_outhit _returnvalue_4) (`KismetSystemLibrary.LineTraceSingle` _returnvalue_3 (+ _returnvalue_3 (* (`self.GetForwardVector` _camera) (`self.Range`))) "TraceTypeQuery1" false (`|MakeArray` _returnvalue_2 (`Actor.GetParentActor` _returnvalue_2)) "ForDuration" true (struct :`R` 1.0 :`A` 1.0) (struct :`G` 1.0 :`A` 1.0) 0.1))
        (if _returnvalue_4
          (bind (_bblockinghit _binitialoverlap _time _distance _location _impactpoint _normal _impactnormal _physmat _hitactor _hitcomponent _hitbonename _bonename _hititem _elementindex _faceindex _tracestart _traceend) (`GameplayStatics.BreakHitResult` _outhit))
          (bind _returnvalue_5 (- _traceend _tracestart))
          (`NiagaraFunctionLibrary.SpawnSystemAtLocation` "/Game/FX/NS_BulletHit.NS_BulletHit" _impactpoint (`KismetMathLibrary.Conv_VectorToRotator` (`KismetMathLibrary.RotateAngleAxis` (`KismetMathLibrary.NegateVector` _returnvalue_5) 180.0 _normal)))
          (`|ExecutionSequence`
            (:`then_0`
              (if (`self.IsSimulatingPhysics` _hitcomponent "None")
                (bind _returnvalue_6 (`Actor.GetComponentByClass` _hitactor "/Game/Characters/Blueprints/BPC_Health.BPC_Health_C"))
                (`/Engine/EditorBlueprintResources/StandardMacros.IsValid` _returnvalue_6
                  (:`Is Valid`
                    (if (not (`/Game/Characters/Blueprints/BPC_Health.OverrideGunRecoil` _returnvalue_6))
                      (`PrimitiveComponent.AddForceAtLocation` _hitcomponent (* (`KismetMathLibrary.Normal` _returnvalue_5) (`KismetMathLibrary.Conv_DoubleToVector` 1000000.0)) _impactpoint "None" :!label _label)))
                  (:`Is Not Valid`
                    (goto _label)))))
            (:`then_1`
              (message `/Game/Characters/Blueprints/BPI_Lifecycle.TakeDamage` _hitactor (`self.Damage`) _outhit (select `bool` (`KismetSystemLibrary.IsValid` (`self.Camera`)) :`false` _returnvalue :`true` (`Actor.GetParentActor` _returnvalue)))))))
      (:`then_1`
        (`NiagaraFunctionLibrary.SpawnSystemAttached` "/Game/FX/NS_MuzzleFlash.NS_MuzzleFlash" self "None" (0.0 0.0 0.0) (struct) "SnapToTarget" true))
      (:`then_2`
        (`/Engine/EditorBlueprintResources/StandardMacros.DecrementInt` _curammo
          (:`  `
            (if (<= _curammo 0)
              (`self.Reload`)
              (else
                (set `self.CanShoot` false)
                (`KismetSystemLibrary.Delay` (/ 1.0 (`self.FireRate`)))
                (set `self.CanShoot` true))))))
      (:`then_3`
        (set `self.RecoilPos` (+ (`self.RecoilPos`) (-20.0 0.0 5.0)))))))