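; Component that lets the player take control of its owning pawn, likely a ship, and return to their character.
; Interact possesses the owner, freezes and attaches the previous pawn, and adds an input mapping context.
; IA_Interact reverses this, restoring walking and leveling pawn rotation and view roll.
; Freelook applies clamped offsets to the owner's camera, and releasing the toggle eases it back to the default via a looping timer lerp.
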(event `self.ReceiveBeginPlay`
  (`KismetSystemLibrary.Delay` 0.2)
  (set `self.DefaultCameraRot` (`SceneComponent.RelativeRotation` (`Actor.GetComponentByClass` (`self.GetOwner`) "/Script/Engine.CameraComponent"))))

(event `/Game/Items/BPI_Interactable.Interact`
  (bind _aspawn (cast `Pawn` (`self.GetOwner`)))
  (set `self.PrevPawn` (`GameplayStatics.GetPlayerPawn` 0))
  (`Controller.Possess` (`GameplayStatics.GetPlayerController` 0) _aspawn)
  (`CharacterMovementComponent.DisableMovement` (`Actor.GetComponentByClass` (`self.PrevPawn`) "/Script/Engine.CharacterMovementComponent"))
  (`Actor.K2_AttachToComponent` (`self.PrevPawn`) self "None" "KeepWorld" "KeepWorld" "KeepWorld" true)
  (`EnhancedInputSubsystemInterface.AddMappingContext` (pcsubsystem `EnhancedInputLocalPlayerSubsystem` (`GameplayStatics.GetPlayerController` 0)) (`self.InputMappingContext`) 4 (struct)))

(event `EnhancedInput|/Game/Player/Input/Actions/IA_Interact`
  (params (ActionValue :type Boolean) (ElapsedSeconds :type "Float (double-precision)") (TriggeredSeconds :type "Float (double-precision)") (InputAction :type "InputAction Object Reference" :default "/Game/Player/Input/Actions/IA_Interact.IA_Interact"))
  (bind _returnvalue (`GameplayStatics.GetPlayerController` 0))
  (bind _prevpawn (`self.PrevPawn`))
  (bind (_returnvalue_roll _returnvalue_pitch _returnvalue_yaw) (`KismetMathLibrary.BreakRotator` (`Controller.GetControlRotation` _returnvalue)))
  (:`Triggered`
    (if ActionValue
      (`Controller.Possess` (`GameplayStatics.GetPlayerController` 0) (`self.PrevPawn`))
      (`Actor.K2_DetachFromActor` _prevpawn "KeepWorld" "KeepWorld" "KeepWorld")
      (`CharacterMovementComponent.SetMovementMode` (`Actor.GetComponentByClass` _prevpawn "/Script/Engine.CharacterMovementComponent") "MOVE_Walking" 0)
      (`Actor.K2_SetActorRotation` :`self` _prevpawn)
      (`Controller.SetControlRotation` _returnvalue (`KismetMathLibrary.MakeRotator` 0.0 _returnvalue_pitch _returnvalue_yaw))
      (`EnhancedInputSubsystemInterface.RemoveMappingContext` (pcsubsystem `EnhancedInputLocalPlayerSubsystem` (`GameplayStatics.GetPlayerController` 0)) (`self.InputMappingContext`) (struct)))))

(event `EnhancedInput|/Game/Ships/Input/IA_Freelook`
  (params (ActionValue :type "Vector2D Structure") (ElapsedSeconds :type "Float (double-precision)") (TriggeredSeconds :type "Float (double-precision)") (InputAction :type "InputAction Object Reference" :default "/Game/Ships/Input/IA_Freelook.IA_Freelook"))
  (bind (_camerarot_roll _camerarot_pitch _camerarot_yaw) (`KismetMathLibrary.BreakRotator` (`self.CameraRot`)))
  (:`Triggered`
    (bind _output_get (set `self.CameraRot` (`KismetMathLibrary.MakeRotator` 0.0 (`KismetMathLibrary.FClamp` (+ _camerarot_pitch (* ActionValue_Y -1.0)) -45.0 45.0) (`KismetMathLibrary.FClamp` (+ _camerarot_yaw ActionValue_X) -45.0 45.0))))
    (`self.K2_SetRelativeRotation` (`Actor.GetComponentByClass` (`self.GetOwner`) "/Script/Engine.CameraComponent") (`KismetMathLibrary.ComposeRotators` _output_get (`self.DefaultCameraRot`)) false false)))

(event `EnhancedInput|/Game/Ships/Input/IA_FreelookToggle`
  (params (ActionValue :type Boolean) (ElapsedSeconds :type "Float (double-precision)") (TriggeredSeconds :type "Float (double-precision)") (InputAction :type "InputAction Object Reference" :default "/Game/Ships/Input/IA_FreelookToggle.IA_FreelookToggle"))
  (:`Completed`
    (if true
      (set `self.CameraRot` (struct))
      (bind _returnvalue (`KismetSystemLibrary.K2_SetTimerDelegate` (delegate `LerpCameraBack`) (`GameplayStatics.GetWorldDeltaSeconds`) true))
      (set `self.CameraReturnTimer` _returnvalue))))

(event `LerpCameraBack`
  (bind _defaultcamerarot (`self.DefaultCameraRot`))
  (bind _returnvalue (`Actor.GetComponentByClass` (`self.GetOwner`) "/Script/Engine.CameraComponent"))
  (bind _returnvalue_2 (`KismetMathLibrary.RLerp` (`SceneComponent.RelativeRotation` _returnvalue) _defaultcamerarot 0.1))
  (`self.K2_SetRelativeRotation` _returnvalue _returnvalue_2 false false)
  (if (< (`KismetMathLibrary.VSize` (`KismetMathLibrary.MakeVector` (.roll (`KismetMathLibrary.NormalizedDeltaRotator` _defaultcamerarot _returnvalue_2)) (.pitch (`KismetMathLibrary.NormalizedDeltaRotator` _defaultcamerarot _returnvalue_2)) (.yaw (`KismetMathLibrary.NormalizedDeltaRotator` _defaultcamerarot _returnvalue_2)))) 0.5)
    (`KismetSystemLibrary.K2_ClearAndInvalidateTimerHandle` (`self.CameraReturnTimer`))))