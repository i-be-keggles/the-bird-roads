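; AI controller that flies a BP_Airship around a looping set of three hard-coded debug waypoints.
; Each tick it steers the joystick from the look-at rotation delta, holds constant throttle, feeds back roll and lifts toward the target altitude.
; A forward sphere trace toward the nose, capped by distance to the waypoint, flags obstacles, overriding altitude control with upward lift to climb over them.
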(event `DebugSetDestination`
  (bind _destinationindexdebug (`self.DestinationIndexDebug`))
  (bind _array (`|MakeArray` (`KismetMathLibrary.MakeVector` 0.0 0.0 2500.0) (`KismetMathLibrary.MakeVector` 22000.0 14000.0 8000.0) (`KismetMathLibrary.MakeVector` 46000.0 -8000.0 6000.0)))
  (set `self.TargetDestination` (`|GetArrayItem` _array _destinationindexdebug))
  (bind _output_get (set `self.DestinationIndexDebug` (+ _destinationindexdebug 1)))
  (if (>= _output_get (`KismetArrayLibrary.Array_Length` _array))
    (set `self.DestinationIndexDebug` 0)))

(event `self.ReceiveBeginPlay`
  (bind _asbp_airship (cast `/Game/Ships/Blueprints/BP_Airship` (`self.K2_GetPawn`)))
  (set `self.Airship` _asbp_airship)
  (`self.DebugSetDestination`))

(event `self.ReceiveTick`
  (params (DeltaSeconds :type "Float (single-precision)"))
  (bind _returnvalue (`self.K2_GetPawn`))
  (bind _airship (`self.Airship`))
  (bind _airship_2 (`self.Airship`))
  (bind (_targetdestination_x _targetdestination_y _targetdestination_z) (`KismetMathLibrary.BreakVector` (`self.TargetDestination`)))
  (bind _airship_3 (`self.Airship`))
  (bind _root (`/Game/Ships/Blueprints/BP_Airship.Root` (`self.Airship`)))
  (bind _root_2 (`/Game/Ships/Blueprints/BP_Airship.Root` (`self.Airship`)))
  (bind _returnvalue_roll (`KismetMathLibrary.BreakRotator` (`SceneComponent.K2_GetComponentRotation` (`/Game/Ships/Blueprints/BP_Airship.Root` _airship_2))))
  (bind (_returnvalue_x _returnvalue_y _returnvalue_z) (`KismetMathLibrary.BreakVector` (`SceneComponent.K2_GetComponentLocation` (`/Game/Ships/Blueprints/BP_Airship.Root` _airship_3))))
  (bind _returnvalue_2 (`SceneComponent.K2_GetComponentLocation` _root))
  (`KismetSystemLibrary.DrawDebugSphere` (`self.TargetDestination`) 100.0 12 (struct :`G` 0.380255 :`B` 1.0 :`A` 1.0) 0.1)
  (`|ExecutionSequence`
    (:`then_0`
      ;[1 1 1] Destination Check
      (if (<= (`KismetMathLibrary.Vector_Distance` (`SceneComponent.K2_GetComponentLocation` (`/Game/Ships/Blueprints/BP_Airship.Root` (`self.Airship`))) (`self.TargetDestination`)) 2000.0)
        (`self.DebugSetDestination`)))
    (:`then_1`
      ;[1 1 1] Turning
      (set `/Game/Ships/Blueprints/BP_Airship.JoyStick` (`KismetMathLibrary.ClampVectorSize` (`KismetMathLibrary.MakeVector` (.yaw (`KismetMathLibrary.NormalizedDeltaRotator` (`KismetMathLibrary.FindLookAtRotation` (`SceneComponent.K2_GetComponentLocation` _root_2) (`self.TargetDestination`)) (`SceneComponent.K2_GetComponentRotation` _root_2))) (* -1.0 (.pitch (`KismetMathLibrary.NormalizedDeltaRotator` (`KismetMathLibrary.FindLookAtRotation` (`SceneComponent.K2_GetComponentLocation` _root_2) (`self.TargetDestination`)) (`SceneComponent.K2_GetComponentRotation` _root_2))))) 0.0 1.0) (`self.Airship`)))
    (:`then_2`
      ;[1 1 1] Throttle
      (set `/Game/Ships/Blueprints/BP_Airship.Throttle` 0.7 _airship)
      (`/Game/Ships/Blueprints/BP_Airship.MoveForward` _airship 1.0))
    (:`then_3`
      ;[1 1 1] Roll
      (`/Game/Ships/Blueprints/BP_Airship.Roll` _airship_2 (* _returnvalue_roll 1.0 0.1)))
    (:`then_4`
      ;[1 1 1] Lift
      (if (not (`self.Avoiding`))
        (`/Game/Ships/Blueprints/BP_Airship.Lift` _airship_3 (- _targetdestination_z _returnvalue_z))))
    (:`then_5`
      ;[1 1 1] Avoidance
      (bind _output_get (set `self.SelfActors` (`self.GetAllChildActors` _returnvalue true)))
      (`KismetArrayLibrary.Array_Add` _output_get _returnvalue)
      (bind (_outhit _returnvalue_3) (`KismetSystemLibrary.SphereTraceSingle` _returnvalue_2 (+ _returnvalue_2 (* (`SceneComponent.GetForwardVector` _root) (`KismetMathLibrary.FMin` 50000.0 (`KismetMathLibrary.Vector_Distance` _returnvalue_2 (`self.TargetDestination`))))) 900.0 "TraceTypeQuery1" false (`self.SelfActors`)))
      (bind _output_get_2 (set `self.Avoiding` _returnvalue_3))
      (if _output_get_2
        (`/Game/Ships/Blueprints/BP_Airship.Lift` (`self.Airship`) 1.0)))))

(fn `UserConstructionScript`)