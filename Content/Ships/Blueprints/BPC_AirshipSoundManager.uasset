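; Actor component that manages the propeller-driven engine audio of its owning BP_Airship.
; HandleMovementTick, not called within this file, smooths strafe input times throttle into the ship audio's Intensity parameter and sets volume from the propeller ratio.
; A looping one-second timer restarts stopped audio when the player pawn is within attenuation falloff distance of the visual ship, printing a debug message.
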(event `self.ReceiveBeginPlay`
  (bind _asbp_airship (cast `/Game/Ships/Blueprints/BP_Airship` (`self.GetOwner`)))
  (set `self.Airship` _asbp_airship)
  (`KismetSystemLibrary.K2_SetTimerDelegate` (delegate `PlayerCheckTick`) 1.0 true))

(event `HandleMovementTick`
  (bind _airship (`self.Airship`))
  (bind _strafeinput_x (`KismetMathLibrary.BreakVector` (`/Game/Ships/Blueprints/BP_Airship.StrafeInput` _airship)))
  (bind _shipaudio (`/Game/Ships/Blueprints/BP_Airship.ShipAudio` _airship))
  (bind _output_get (set `self.SoundIntensity` (`KismetMathLibrary.Lerp` (`self.SoundIntensity`) (* _strafeinput_x (`/Game/Ships/Blueprints/BP_Airship.Throttle` _airship)) (* (`GameplayStatics.GetWorldDeltaSeconds`) 1.0))))
  (`AudioParameterControllerInterface.SetFloatParameter` _shipaudio "Intensity" _output_get)
  (`AudioComponent.SetVolumeMultiplier` _shipaudio (`/Game/Ships/Blueprints/BP_Airship.PropellorRatio` _airship)))

(event `PlayerCheckTick`
  (bind _airship (`self.Airship`))
  (bind _shipaudio (`/Game/Ships/Blueprints/BP_Airship.ShipAudio` (`self.Airship`)))
  (bind (_attenuation_battenuate _attenuation_bspatialize _attenuation_battenuatewithlpf _attenuation_benablelistenerfocus _attenuation_benablefocusinterpolation _attenuation_benableocclusion _attenuation_busecomplexcollisionforocclusion _attenuation_benablereverbsend _attenuation_benablepriorityattenuation _attenuation_bapplynormalizationtostereosounds _attenuation_benablelogfrequencyscaling _attenuation_benablesubmixsends _attenuation_benablesourcedataoverride _attenuation_benablesendtoaudiolink _attenuation_spatializationalgorithm _attenuation_audiolinksettingsoverride _attenuation_binauralradius _attenuation_customlowpassairabsorptioncurve _attenuation_customhighpassairabsorptioncurve _attenuation_absorptionmethod _attenuation_occlusiontracechannel _attenuation_reverbsendmethod _attenuation_priorityattenuationmethod _attenuation_nonspatializedradiusstart _attenuation_nonspatializedradiusend _attenuation_nonspatializedradiusmode _attenuation_stereospread _attenuation_lpfradiusmin _attenuation_lpfradiusmax _attenuation_lpffrequencyatmin _attenuation_lpffrequencyatmax _attenuation_hpffrequencyatmin _attenuation_hpffrequencyatmax _attenuation_focusazimuth _attenuation_nonfocusazimuth _attenuation_focusdistancescale _attenuation_nonfocusdistancescale _attenuation_focuspriorityscale _attenuation_nonfocuspriorityscale _attenuation_focusvolumeattenuation _attenuation_nonfocusvolumeattenuation _attenuation_focusattackinterpspeed _attenuation_focusreleaseinterpspeed _attenuation_occlusionlowpassfilterfrequency _attenuation_occlusionvolumeattenuation _attenuation_occlusioninterpolationtime _attenuation_reverbwetlevelmin _attenuation_reverbwetlevelmax _attenuation_reverbdistancemin _attenuation_reverbdistancemax _attenuation_manualreverbsendlevel _attenuation_priorityattenuationmin _attenuation_priorityattenuationmax _attenuation_priorityattenuationdistancemin _attenuation_priorityattenuationdistancemax _attenuation_manualpriorityattenuation _attenuation_customreverbsendcurve _attenuation_submixsendsettings _attenuation_custompriorityattenuationcurve _attenuation_pluginsettings _attenuation_distancealgorithm _attenuation_attenuationshape _attenuation_falloffmode _attenuation_dbattenuationatmax _attenuation_attenuationshapeextents _attenuation_coneoffset _attenuation_falloffdistance) (break `SoundAttenuationSettings` (`SoundAttenuation.Attenuation` (`AudioComponent.AttenuationSettings` (`/Game/Ships/Blueprints/BP_Airship.ShipAudio` _airship)))))
  (if (< (`KismetMathLibrary.Vector_Distance` (`Actor.K2_GetActorLocation` (`GameplayStatics.GetPlayerPawn` 0)) (`SceneComponent.K2_GetComponentLocation` (`/Game/Ships/Blueprints/BP_Airship.VisualShip` _airship))) _attenuation_falloffdistance)
    (if (not (`AudioComponent.IsPlaying` _shipaudio))
      (`AudioComponent.Play` _shipaudio 0.0)
      (`KismetSystemLibrary.PrintString` "Restarting ship audio"))))