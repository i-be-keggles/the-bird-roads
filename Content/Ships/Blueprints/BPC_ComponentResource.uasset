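; Actor component that gives a ship component (BP_ShipComponent) a resource pool shown on its gauge widget.
; On BeginPlay it caches the owning ship component and, after a short delay, sets the initial gauge percentage.
; Drain and Add change the clamped value by a multiplier times RateOfChange and update the gauge, only while that widget is valid.
; Reaching empty or full fires the OnResourceDepleted or OnResourceFilled dispatcher.
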(event `self.ReceiveBeginPlay`
  (bind _asbp_ship_component (cast `/Game/Ships/Blueprints/BP_ShipComponent` (`self.GetOwner`)))
  (bind _output_get (set `self.Component` _asbp_ship_component))
  (`KismetSystemLibrary.Delay` 0.1)
  (`/Game/UI/WBP_ResourceGageDebug.SetPercent` (`/Game/Ships/Blueprints/BP_ShipComponent.GaugeWidget` _output_get) (/ (`self.CurResource`) (`self.MaxResource`))))

(event `DrainResource`
  (params (AmountMultiplier :type "Float (double-precision)" :default 1.0))
  (`/Engine/EditorBlueprintResources/StandardMacros.IsValid` (`/Game/Ships/Blueprints/BP_ShipComponent.GaugeWidget` (`self.Component`))
    (:`Is Valid`
      (bind _output_get (set `self.CurResource` (`KismetMathLibrary.FMax` (- (`self.CurResource`) (* AmountMultiplier (`self.RateOfChange`))))))
      (`/Game/UI/WBP_ResourceGageDebug.SetPercent` (`/Game/Ships/Blueprints/BP_ShipComponent.GaugeWidget` (`self.Component`)) (/ _output_get (`self.MaxResource`)))
      (if (<= _output_get 0.0)
        (`self.ResourceDepleted`)))))

(event `AddResource`
  (params (AmountMultiplier :type "Float (double-precision)" :default 1.0))
  (bind _maxresource (`self.MaxResource`))
  (`/Engine/EditorBlueprintResources/StandardMacros.IsValid` (`/Game/Ships/Blueprints/BP_ShipComponent.GaugeWidget` (`self.Component`))
    (:`Is Valid`
      (bind _output_get (set `self.CurResource` (`KismetMathLibrary.FMin` (+ (`self.CurResource`) (* AmountMultiplier (`self.RateOfChange`))) _maxresource)))
      (`/Game/UI/WBP_ResourceGageDebug.SetPercent` (`/Game/Ships/Blueprints/BP_ShipComponent.GaugeWidget` (`self.Component`)) (/ _output_get (`self.MaxResource`)))
      (if (>= _output_get _maxresource)
        (`self.ResourceFilled`)))))

(event `ResourceDepleted`
  (`self.OnResourceDepleted`))

(event `ResourceFilled`
  (`self.OnResourceFilled`))