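; Scene component that represents a gas leak on an airship, dragging the ship down along world Z while it exists.
; On BeginPlay it caches its BP_Airship owner and attaches a gas leak particle system at its own location.
; Each tick it applies Force negated on Z to the airship's root as an acceleration, independent of mass.
; RemoveLeak destroys the particles and the component.
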(event `self.ReceiveBeginPlay`
  (bind _asbp_airship (cast `/Game/Ships/Blueprints/BP_Airship` (`self.GetOwner`)))
  (set `self.Airship` _asbp_airship)
  (bind _returnvalue (`NiagaraFunctionLibrary.SpawnSystemAttached` "/Game/FX/NS_GasLeak.NS_GasLeak" self "None" (`self.K2_GetComponentLocation`) (`self.K2_GetComponentRotation`) "KeepWorldPosition"))
  (set `self.Particles` _returnvalue))

(event `self.ReceiveTick`
  (params (DeltaSeconds :type "Float (single-precision)"))
  (`PrimitiveComponent.AddForce` (`/Game/Ships/Blueprints/BP_Airship.Root` (`self.Airship`)) (`KismetMathLibrary.MakeVector` 0.0 0.0 (* (`self.Force`) -1.0)) "None" true))

(event `RemoveLeak`
  (`self.K2_DestroyComponent` (`self.Particles`))
  (`self.K2_DestroyComponent` self))