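; Component that lets the player take control of a ship-related pawn (its owner or owner's parent actor) and later return to their previous pawn.
; Interact, refused when AI-enabled or neutralised with health, possesses the pawn, hides and attaches the player's pawn, and adds an input context.
; IA_Interact reverses this.
; Freelook rotates the camera within clamped limits, then a looping timer eases it back to default on release.
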(event `SetAIEnabled`
  (params (Enabled :type Boolean))
  (set `self.AIEnabled` Enabled))

(event `self.ReceiveBeginPlay`
  (bind _returnvalue (`self.GetOwner`))
  (bind _returnvalue_2 (`self.GetOwner`))
  (bind _returnvalue_3 (`Actor.GetComponentByClass` _returnvalue "/Script/Engine.CameraComponent"))
  (bind _returnvalue_4 (`Actor.GetComponentByClass` (`Actor.GetParentActor` _returnvalue) "/Script/Engine.CameraComponent"))
  (bind _aspawn (cast `Pawn` _returnvalue_2)
    (:`then`
      (set `self.Pawn` _aspawn))
    (:`CastFailed`
      (bind _aspawn_2 (cast `Pawn` (`Actor.GetParentActor` _returnvalue_2)))
      (set `self.Pawn` _aspawn_2)))
  (`|ExecutionSequence`
    (:`then_1`
      (`KismetSystemLibrary.Delay` 0.2)
      (`/Engine/EditorBlueprintResources/StandardMacros.IsValid` _returnvalue_3
        (:`Is Valid`
          (set `self.Camera` _returnvalue_3)
          (set `self.DefaultCameraRot` (`SceneComponent.RelativeRotation` _returnvalue_3)))
        (:`Is Not Valid`
          (set `self.Camera` _returnvalue_4)
          (set `self.DefaultCameraRot` (`SceneComponent.RelativeRotation` _returnvalue_4)))))))

(event `/Game/Items/BPI_Interactable.Interact`
  (params (Held :type Boolean))
  (bind _returnvalue (`self.GetOwner`))
  (bind _health (message `/Game/Ships/Components/BPI_ShipComponent.GetMaxHealth` _returnvalue))
  (bind _isneutralised (message `/Game/Ships/Components/BPI_ShipComponent.IsNeutralised` _returnvalue))
  (if (or (and _isneutralised (> _health 0)) (`self.AIEnabled`))
    (`KismetSystemLibrary.PrintString` "nO")
    (else
      (set `self.PrevPawn` (`GameplayStatics.GetPlayerPawn` 0))
      (`Controller.Possess` (`GameplayStatics.GetPlayerController` 0) (`self.Pawn`))
      (`CharacterMovementComponent.DisableMovement` (`Actor.GetComponentByClass` (`self.PrevPawn`) "/Script/Engine.CharacterMovementComponent"))
      (`Actor.K2_AttachToComponent` (`self.PrevPawn`) self "None" "KeepWorld" "KeepWorld" "KeepWorld" true)
      (`EnhancedInputSubsystemInterface.AddMappingContext` (pcsubsystem `EnhancedInputLocalPlayerSubsystem` (`GameplayStatics.GetPlayerController` 0)) (`self.InputMappingContext`) 4 (struct))
      (`self.OnPlayerPossessionChanged`)
      (set `self.IsPossessedByPlayer` true)
      (`Actor.EnableInput` (`self.GetOwner`) (`GameplayStatics.GetPlayerController` 0))
      (`Actor.SetActorHiddenInGame` (`self.PrevPawn`) true))))

(event `EnhancedInput|/Game/Player/Input/Actions/IA_Interact`
  (params (ActionValue :type Boolean) (ElapsedSeconds :type "Float (double-precision)") (TriggeredSeconds :type "Float (double-precision)") (InputAction :type "InputAction Object Reference" :default "/Game/Player/Input/Actions/IA_Interact.IA_Interact"))
  (bind _returnvalue (`GameplayStatics.GetPlayerController` 0))
  (bind _prevpawn (`self.PrevPawn`))
  (bind (_returnvalue_roll _returnvalue_pitch _returnvalue_yaw) (`KismetMathLibrary.BreakRotator` (`Controller.GetControlRotation` _returnvalue)))
  (:`Triggered`
    (if ActionValue
      (`Controller.Possess` (`GameplayStatics.GetPlayerController` 0) (`self.PrevPawn`))
      (`Actor.K2_DetachFromActor` _prevpawn "KeepWorld" "KeepWorld" "KeepWorld")
      (`CharacterMovementComponent.SetMovementMode` (`Actor.GetComponentByClass` _prevpawn "/Script/Engine.CharacterMovementComponent") "MOVE_Walking" 0)
      (`Actor.K2_SetActorRotation` :`self` _prevpawn)
      (`Controller.SetControlRotation` _returnvalue (`KismetMathLibrary.MakeRotator` 0.0 _returnvalue_pitch _returnvalue_yaw))
      (`self.K2_SetRelativeRotation` (`Actor.GetComponentByClass` _prevpawn "/Script/Engine.CameraComponent") (`KismetMathLibrary.MakeRotator` 0.0 _returnvalue_pitch) false false)
      (`EnhancedInputSubsystemInterface.RemoveMappingContext` (pcsubsystem `EnhancedInputLocalPlayerSubsystem` (`GameplayStatics.GetPlayerController` 0)) (`self.InputMappingContext`) (struct))
      (`self.OnPlayerPossessionChanged`)
      (set `self.IsPossessedByPlayer` false)
      (`Actor.DisableInput` (`self.GetOwner`) (`GameplayStatics.GetPlayerController` 0))
      (`Actor.SetActorHiddenInGame` (`self.PrevPawn`) false))))

(event `EnhancedInput|/Game/Ships/Input/IA_Freelook`
  (params (ActionValue :type "Vector2D Structure") (ElapsedSeconds :type "Float (double-precision)") (TriggeredSeconds :type "Float (double-precision)") (InputAction :type "InputAction Object Reference" :default "/Game/Ships/Input/IA_Freelook.IA_Freelook"))
  (bind (_camerarot_roll _camerarot_pitch _camerarot_yaw) (`KismetMathLibrary.BreakRotator` (`self.CameraRot`)))
  (:`Triggered`
    (bind _output_get (set `self.CameraRot` (`KismetMathLibrary.MakeRotator` 0.0 (`KismetMathLibrary.FClamp` (+ _camerarot_pitch (* ActionValue_Y -1.0)) -45.0 45.0) (`KismetMathLibrary.FClamp` (+ _camerarot_yaw ActionValue_X) -65.0 65.0))))
    (`self.K2_SetRelativeRotation` (`self.Camera`) (`KismetMathLibrary.ComposeRotators` _output_get (`self.DefaultCameraRot`)) false false)))

(event `EnhancedInput|/Game/Ships/Input/IA_FreelookToggle`
  (params (ActionValue :type Boolean) (ElapsedSeconds :type "Float (double-precision)") (TriggeredSeconds :type "Float (double-precision)") (InputAction :type "InputAction Object Reference" :default "/Game/Ships/Input/IA_FreelookToggle.IA_FreelookToggle"))
  (:`Completed`
    (if true
      (set `self.CameraRot` (struct))
      (bind _returnvalue (`KismetSystemLibrary.K2_SetTimerDelegate` (delegate `LerpCameraBack`) (`GameplayStatics.GetWorldDeltaSeconds`) true))
      (set `self.CameraReturnTimer` _returnvalue))))

(event `LerpCameraBack`
  (bind _defaultcamerarot (`self.DefaultCameraRot`))
  (bind _camera (`self.Camera`))
  (bind _returnvalue (`KismetMathLibrary.RLerp` (`SceneComponent.RelativeRotation` _camera) _defaultcamerarot 0.1))
  (`self.K2_SetRelativeRotation` _camera _returnvalue false false)
  (if (< (`KismetMathLibrary.VSize` (`KismetMathLibrary.MakeVector` (.roll (`KismetMathLibrary.NormalizedDeltaRotator` _defaultcamerarot _returnvalue)) (.pitch (`KismetMathLibrary.NormalizedDeltaRotator` _defaultcamerarot _returnvalue)) (.yaw (`KismetMathLibrary.NormalizedDeltaRotator` _defaultcamerarot _returnvalue)))) 0.5)
    (`KismetSystemLibrary.K2_ClearAndInvalidateTimerHandle` (`self.CameraReturnTimer`))))