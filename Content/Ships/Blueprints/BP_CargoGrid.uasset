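; BP_CargoGrid is a ship cargo grid actor that holds items in cells, stored in a flat array indexed by X/Y.
; The construction script builds a cube marker per cell, and helpers convert between world positions and slots.
; TryAddItem rejects occupied cells, otherwise disables physics, attaches the item at the cell center and rounds yaw to 90 degrees.
; RemoveItem only removes the array entry, shifting later indices, without detaching the item.
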(event `self.ReceiveBeginPlay`
  ;[1 1 1] PopulateArray
  (for _ (range (`self.SizeX`))
    (for _ (range (`self.SizeY`))
      (`KismetArrayLibrary.Array_Add` (`self.Items`)))))

(event `TryAddItem`
  (params (Item :type "/Game/Items/BP_Carryable Object Reference") (PosX :type Integer) (PosY :type Integer))
  (bind _staticmesh (`/Game/Items/BP_Item.StaticMesh` Item))
  (bind _staticmesh_2 (`/Game/Items/BP_Item.StaticMesh` Item))
  (bind (_relativerotation_roll _relativerotation_pitch _relativerotation_yaw) (`KismetMathLibrary.BreakRotator` (`SceneComponent.RelativeRotation` _staticmesh)))
  (bind _index (`self.CoordsToIndex` PosX PosY))
  (if (== (`|GetArrayItem` (`self.Items`) _index) null)
    (`KismetArrayLibrary.Array_Set` (`self.Items`) _index Item)
    (set `/Game/Items/BP_Carryable.CargoGrid` self Item)
    ;[1 1 1] Attach
    (`PrimitiveComponent.SetSimulatePhysics` _staticmesh_2 false)
    (`self.K2_AttachToActor` Item self "None" "SnapToTarget" "SnapToTarget" "KeepWorld" true)
    (`SceneComponent.K2_AttachToComponent` _staticmesh_2 (`/Game/Items/BP_Item.DefaultSceneRoot` Item) "None" "SnapToTarget" "KeepWorld" "KeepWorld" true)
    (bind _position (`self.GetSlotWorldTransform` PosX PosY))
    (`SceneComponent.K2_SetWorldLocation` _staticmesh _position false false)
    (`SceneComponent.K2_SetRelativeRotation` _staticmesh (`KismetMathLibrary.MakeRotator` 0.0 0.0 (`KismetMathLibrary.Conv_IntToDouble` (* (`KismetMathLibrary.Round` (/ _relativerotation_yaw 90.0)) 90))) false false)
    (else
      (`KismetSystemLibrary.PrintString` "Space occupied"))))

(event `RemoveItem`
  (params (Item :type "/Game/Items/BP_Carryable Object Reference"))
  (`KismetArrayLibrary.Array_RemoveItem` (`self.Items`) Item))

(fn `CoordsToIndex`
  (params (X :type Integer) (Y :type Integer))
  (returns (Index :type Integer))
  (return (+ X (* Y (`self.SizeX`)))))

(fn `GetSlotFromWorldPos`
  (params (`World Position` :type "Vector Structure"))
  (returns (X :type Integer) (Y :type Integer))
  (bind _cellsize (`self.CellSize`))
  (bind (_returnvalue_x _returnvalue_y) (`KismetMathLibrary.BreakVector` (`KismetMathLibrary.InverseTransformLocation` (`self.GetTransform`) `World Position`)))
  (return (`KismetMathLibrary.FTrunc` (/ _returnvalue_x _cellsize)) (`KismetMathLibrary.FTrunc` (/ _returnvalue_y _cellsize))))

(fn `GetSlotWorldTransform`
  (params (X :type Integer) (Y :type Integer))
  (returns (Position :type "Vector Structure"))
  (bind _cellsize (`self.CellSize`))
  (bind _returnvalue (/ (`self.CellSize`) 2.0))
  (return (`KismetMathLibrary.TransformLocation` (`self.GetTransform`) (`KismetMathLibrary.MakeVector` (+ (* X _cellsize) _returnvalue) (+ (* Y _cellsize) _returnvalue) _returnvalue))))

(fn `UserConstructionScript`
  (bind _cellsize (`self.CellSize`))
  (bind _returnvalue (/ (`self.CellSize`) 2.0))
  (for _index (range (`self.SizeX`))
    (for _index_2 (range (`self.SizeY`))
      (bind _returnvalue_2 (`AddComponent|NODE_AddStaticMeshComponent-0` :`RelativeTransform` (`KismetMathLibrary.MakeTransform` (`KismetMathLibrary.MakeVector` (+ (* _index_2 _cellsize) _returnvalue) (+ (* _index _cellsize) _returnvalue)) (struct) (0.4 0.4 0.05))))
      (`StaticMeshComponent.SetStaticMesh` _returnvalue_2 "/Game/ArtPrototyping/Ships/250cmcube.250cmcube"))))