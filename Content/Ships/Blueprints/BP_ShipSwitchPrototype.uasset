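; Prototype ship-switching actor that lets the player cycle possession between the starting pawn and every BP_Airship in the level.
; On BeginPlay it gathers the airships, gives them one shared throttle widget, adds debug and build-info widgets, enables its own input, and puts the player pawn first in the list.
; SwitchShip possesses the next entry, wrapping to the start, and Info toggles the debug HUD.
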(event `self.ReceiveBeginPlay`
  (bind _outactors (`GameplayStatics.GetAllActorsOfClass` "/Game/Ships/Blueprints/BP_Airship.BP_Airship_C"))
  (set `self.Ships` _outactors)
  (`|ExecutionSequence`
    (:`then_0`
      (bind _returnvalue (`|CreateWidget` "/Game/UI/HUD/WBP_Throttle.WBP_Throttle_C"))
      (`UserWidget.AddToViewport` _returnvalue 0)
      (for _array_element (`self.Ships`)
        (bind _asbp_airship (cast `/Game/Ships/Blueprints/BP_Airship` _array_element))
        (set `/Game/Ships/Blueprints/BP_Airship.ThrottleWidget` _returnvalue _asbp_airship)))
    (:`then_1`
      (bind _returnvalue_2 (`|CreateWidget` "/Game/UI/HUD/WBP_DebugHUD.WBP_DebugHUD_C"))
      (bind _output_get (set `self.DebugHud` _returnvalue_2))
      (`UserWidget.AddToViewport` _output_get 0))
    (:`then_2`
      (`self.EnableInput` (`GameplayStatics.GetPlayerController` 0)))
    (:`then_3`
      (bind _returnvalue_3 (`|CreateWidget` "/Game/UI/HUD/WBP_BuildInfo.WBP_BuildInfo_C"))
      (`UserWidget.AddToViewport` _returnvalue_3 0))
    (:`then_4`
      (`KismetArrayLibrary.Array_Insert` (`self.Ships`) (`GameplayStatics.GetPlayerPawn` 0)))))

(event `InputAction|SwitchShip`
  (params (Key :type "Key Structure"))
  (bind _ships (`self.Ships`))
  (:`Pressed`
    (bind _result (`/Engine/EditorBlueprintResources/StandardMacros.IncrementInt` (`self.CurrentPossesed`))
      (:`  `
        (`|ExecutionSequence`
          (:`then_0`
            (if (>= _result (`KismetArrayLibrary.Array_Length` _ships))
              (set `self.CurrentPossesed` 0)))
          (:`then_1`
            (`Controller.Possess` (`GameplayStatics.GetPlayerController` 0) (`|GetArrayItem` _ships (`self.CurrentPossesed`)))))))))

(event `InputAction|Info`
  (params (Key :type "Key Structure"))
  (:`Pressed`
    (`/Game/UI/HUD/WBP_DebugHUD.ToggleInfo` (`self.DebugHud`))))

(fn `UserConstructionScript`)