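; BP_ShipComponent is a base actor for airship parts that can be switched on or off, hold a resource, take damage and die.
; On BeginPlay it caches its parent BP_Airship and sets up a debug gauge widget with its label and active state.
; Drain and add calls go to BPC_ComponentResource, whose depletion clears the active flag.
; Zero health turns the part off and fires the death notification.
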(event `self.ReceiveBeginPlay`
  (bind _asbp_airship (cast `/Game/Ships/Blueprints/BP_Airship` (`self.GetParentActor`)))
  (set `self.Airship` _asbp_airship)
  (bind _aswbp_resource_gage_debug (cast `/Game/UI/WBP_ResourceGageDebug` (`WidgetComponent.GetWidget` (`self.Widget`))))
  (bind _output_get (set `self.GaugeWidget` _aswbp_resource_gage_debug))
  (`/Game/UI/WBP_ResourceGageDebug.SetLabel` _output_get (`self.Label`))
  (`/Game/UI/WBP_ResourceGageDebug.SetActive` _output_get (`self.Active`)))

(event `TurnOn`
  (bind _output_get (set `self.Active` true))
  (`/Game/UI/WBP_ResourceGageDebug.SetActive` (`self.GaugeWidget`) _output_get)
  (`self.OnTurnedOn`))

(event `TurnOff`
  (bind _output_get (set `self.Active` false))
  (`/Game/UI/WBP_ResourceGageDebug.SetActive` (`self.GaugeWidget`) _output_get)
  (`self.OnTurnedOff`))

(event `/Game/Ships/Blueprints/BPI_ShipComponent.DrainResource`
  (params (Multiplier :type "Float (double-precision)"))
  (`/Game/Ships/Blueprints/BPC_ComponentResource.DrainResource` (`self.BPC_ComponentResource`) Multiplier))

(event `/Game/Ships/Blueprints/BPI_ShipComponent.AddResource`
  (params (Multiplier :type "Float (double-precision)"))
  (`/Game/Ships/Blueprints/BPC_ComponentResource.AddResource` (`self.BPC_ComponentResource`) Multiplier))

(event `self.BPC_ComponentResource.OnResourceDepleted`
  (set `self.Active` false))

(event `/Game/Ships/Blueprints/BPI_ShipComponent.TakeDamage`
  (params (Amount :type Integer) (Hit :type "HitResult Structure"))
  (set `self.PrevHit` Hit)
  (bind _output_get (set `self.Health` (`KismetMathLibrary.Max` (- (`self.Health`) Amount))))
  (if (<= _output_get 0)
    (`self.Die`)))

(event `Die`
  (`self.TurnOff`)
  (`self.OnDeath`))

(fn `HasPrimaryResource`
  (returns (Active :type Boolean))
  (return (> (`/Game/Ships/Blueprints/BPC_ComponentResource.CurResource` (`self.BPC_ComponentResource`)) 0.0)))

(fn `IsActive`
  (returns (Active :type Boolean))
  (return (`self.Active`)))

(fn `UserConstructionScript`)