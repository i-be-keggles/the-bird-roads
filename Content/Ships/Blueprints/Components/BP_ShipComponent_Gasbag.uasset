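; Gasbag ship component for airships that springs a gas leak when it dies.
; On Die, it adds a BPC_GasLeak component to the owning airship, positioned at the previous hit's impact point and oriented along the surface normal.
; The leak attaches to the airship root with world transform preserved, so it stays fixed at the puncture as the ship moves.
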(event `self.Die`
  (bind (_prevhit_bblockinghit _prevhit_binitialoverlap _prevhit_time _prevhit_distance _prevhit_location _prevhit_impactpoint _prevhit_normal _prevhit_impactnormal) (`GameplayStatics.BreakHitResult` (`self.PrevHit`)))
  (bind _returnvalue (`|AddComponentByClass` :`self` (`self.Airship`) :`Class` "/Game/Ships/Blueprints/BPC_GasLeak.BPC_GasLeak_C"))
  (`SceneComponent.K2_SetWorldTransform` _returnvalue (`KismetMathLibrary.MakeTransform` _prevhit_impactpoint (`KismetMathLibrary.Conv_VectorToRotator` _prevhit_impactnormal)) false true)
  (`SceneComponent.K2_AttachToComponent` _returnvalue (`/Game/Ships/Blueprints/BP_Airship.Root` (`self.Airship`)) "None" "KeepWorld" "KeepWorld" "KeepWorld" true))

(fn `UserConstructionScript`
  (`parent.UserConstructionScript`))