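; BP_ShipComponent is an airship component actor with health, an on/off state, a resource and a debug gauge widget.
; It links to its parent BP_Airship, notifying it of hits and using its faction unless overridden.
; Damage drives a dynamic material's Damage parameter; zero health turns the component off once, with broken particles.
; Repair resets that death gate, reactivates the component and clears the particles, while resource depletion clears Active.
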(event `self.ReceiveBeginPlay`
  (bind _returnvalue (`self.GetComponentByClass` "/Script/Engine.SkeletalMeshComponent"))
  (bind _returnvalue_2 (`self.GetComponentByClass` "/Script/Engine.StaticMeshComponent"))
  (`|ExecutionSequence`
    (:`then_0`
      (if true
        (`/Engine/EditorBlueprintResources/StandardMacros.IsValid` _returnvalue_2
          (:`Is Valid`
            (bind _returnvalue_3 (`PrimitiveComponent.CreateDynamicMaterialInstance` _returnvalue_2 0 (`PrimitiveComponent.GetMaterial` _returnvalue_2 0) "None"))
            (set `self.Material` _returnvalue_3))
          (:`Is Not Valid`
            (`/Engine/EditorBlueprintResources/StandardMacros.IsValid` _returnvalue
              (:`Is Valid`
                (bind _returnvalue_4 (`PrimitiveComponent.CreateDynamicMaterialInstance` _returnvalue 0 (`PrimitiveComponent.GetMaterial` _returnvalue 0) "None"))
                (set `self.Material` _returnvalue_4)))))))
    (:`then_1`
      (bind _asbp_airship (cast `/Game/Ships/Blueprints/BP_Airship` (`self.GetParentActor`)))
      (set `self.Airship` _asbp_airship)
      (bind _aswbp_resource_gage_debug (cast `/Game/UI/WBP_ResourceGageDebug` (`WidgetComponent.GetWidget` (`self.Widget`))))
      (bind _output_get (set `self.GaugeWidget` _aswbp_resource_gage_debug))
      (`/Game/UI/WBP_ResourceGageDebug.SetLabel` _output_get (`self.Label`))
      (`/Game/UI/WBP_ResourceGageDebug.SetActive` _output_get (`self.Active`)))))

(event `TurnOn`
  (bind _gaugewidget (`self.GaugeWidget`))
  (`self.OnTurnedOn`)
  (bind _output_get (set `self.Active` true))
  (`/Engine/EditorBlueprintResources/StandardMacros.IsValid` _gaugewidget
    (:`Is Valid`
      (`/Game/UI/WBP_ResourceGageDebug.SetActive` _gaugewidget _output_get))))

(event `TurnOff`
  (bind _gaugewidget (`self.GaugeWidget`))
  (`self.OnTurnedOff`)
  (bind _output_get (set `self.Active` false))
  (`/Engine/EditorBlueprintResources/StandardMacros.IsValid` _gaugewidget
    (:`Is Valid`
      (`/Game/UI/WBP_ResourceGageDebug.SetActive` _gaugewidget _output_get))))

(event `/Game/Ships/Components/BPI_ShipComponent.DrainResource`
  (params (Multiplier :type "Float (double-precision)"))
  (`/Game/Ships/Components/BPC_ComponentResource.DrainResource` (`self.BPC_ComponentResource`) Multiplier))

(event `/Game/Ships/Components/BPI_ShipComponent.AddResource`
  (params (Multiplier :type "Float (double-precision)"))
  (`/Game/Ships/Components/BPC_ComponentResource.AddResource` (`self.BPC_ComponentResource`) Multiplier))

(event `self.BPC_ComponentResource.OnResourceDepleted`
  (set `self.Active` false))

(event `/Game/Ships/Components/BPI_ShipComponent.TakeDamage`
  (params (Amount :type Integer) (Hit :type "HitResult Structure"))
  (if (> (`self.MaxHealth`) 0)
    (set `self.PrevHit` Hit)
    (bind _output_get (set `self.Health` (`KismetMathLibrary.Max` (- (`self.Health`) Amount))))
    (`/Game/Ships/Blueprints/BP_Airship.OnHit` (`self.Airship`))
    (`|ExecutionSequence`
      (:`then_0`
        (`self.UpdateMaterialDamage`))
      (:`then_1`
        (if (<= _output_get 0)
          (`self.Die`))))))

(event `Die`
  (bind _hitvolume (`self.HitVolume`))
  (`/Engine/EditorBlueprintResources/StandardMacros.DoOnce` false :!label _label
    (:`Completed`
      (set `self.HasDied` true)
      (`self.TurnOff`)
      (`self.OnDeath`)
      (bind _returnvalue (`NiagaraFunctionLibrary.SpawnSystemAttached` "/Game/FX/NiagaraSystems/NS_BrokenComponent.NS_BrokenComponent" _hitvolume "None" (`SceneComponent.K2_GetComponentLocation` _hitvolume) (struct) "KeepWorldPosition"))
      (set `self.DeathParticles` _returnvalue))))

(event `/Game/Ships/Components/BPI_ShipComponent.Repair`
  (params (Amount :type Integer))
  (`self.RepairComponent` Amount))

(event `RepairComponent`
  (params (Amount :type Integer))
  (bind _deathparticles (`self.DeathParticles`))
  (if (== Amount 0)
    (set `self.Health` (`self.MaxHealth`))
    (else
      (set `self.Health` (`KismetMathLibrary.Min` (+ Amount (`self.Health`)) (`self.MaxHealth`)))))
  (`|ExecutionSequence`
    (:`then_0`
      (goto _label :!via `Reset`))
    (:`then_1`
      (set `self.HasDied` false)
      (`self.TurnOn`)
      (`self.OnRepair`))
    (:`then_2`
      (`/Engine/EditorBlueprintResources/StandardMacros.IsValid` _deathparticles
        (:`Is Valid`
          (`ActorComponent.K2_DestroyComponent` _deathparticles))))
    (:`then_3`
      (if (>= (`self.Health`) (`self.MaxHealth`))
        (`NiagaraFunctionLibrary.SpawnSystemAtLocation` "/Game/FX/NiagaraSystems/NS_ComponentFix.NS_ComponentFix" (`SceneComponent.K2_GetComponentLocation` (`self.HitVolume`)))))
    (:`then_4`
      (`self.UpdateMaterialDamage`))))

(fn `GetFactionID`
  (returns (FactionID :type Integer))
  (bind _airship (`self.Airship`))
  (bind _factionidoverride (`self.FactionIDOverride`))
  (`/Engine/EditorBlueprintResources/StandardMacros.IsValid` _airship
    (:`Is Valid`
      (return (`KismetMathLibrary.SelectInt` _factionidoverride (`/Game/Ships/Blueprints/BP_Airship.FactionID` _airship) (> _factionidoverride 0))))
    (:`Is Not Valid`
      (return (`self.FactionIDOverride`)))))

(fn `GetMaxHealth`
  (returns (Health :type Integer))
  (return (`self.MaxHealth`)))

(fn `GetShipVelocity`
  (returns (Velocity :type "Vector Structure"))
  (return (`SceneComponent.GetComponentVelocity` (`/Game/Ships/Blueprints/BP_Airship.Root` (`self.Airship`)))))

(fn `HasPrimaryResource`
  (returns (Active :type Boolean))
  (return (> (`/Game/Ships/Components/BPC_ComponentResource.CurResource` (`self.BPC_ComponentResource`)) 0.0)))

(fn `IsActive`
  (returns (Active :type Boolean))
  (return (`self.Active`)))

(fn `IsAttended`
  (returns (IsAttended :type Boolean))
  (return false))

(fn `IsNeutralised`
  (returns (IsNeutralised :type Boolean))
  (return (<= (`self.Health`) 0)))

(fn `UpdateMaterialDamage`
  (bind _material (`self.Material`))
  (`/Engine/EditorBlueprintResources/StandardMacros.IsValid` _material
    (:`Is Valid`
      (`MaterialInstanceDynamic.SetScalarParameterValue` _material "Damage" (- 1.0 (/ (`self.Health`) (`KismetMathLibrary.Conv_IntToDouble` (`self.MaxHealth`))))))))

(fn `UserConstructionScript`)