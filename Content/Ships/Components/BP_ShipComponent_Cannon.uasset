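; Ship cannon component that a character can man, turning on the cannon's AI.
; BeginPlay caches the BPC_Possessable of the Cannon child actor, whose AI state also answers IsAttended.
; Primary interaction enables that AI, disables the character's AI controller and movement, and attaches them to the Pitch socket.
; Secondary interaction only disables the cannon AI, without detaching the character; death fires OnDeath.
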(event `self.Die`
  (`parent.Die`)
  (`self.OnDeath`))

(event `self.ReceiveBeginPlay`
  (`parent.ReceiveBeginPlay`)
  (set `self.Possessable` (`self.GetComponentByClass` (`ChildActorComponent.ChildActor` (`self.Cannon`)) "/Game/Ships/Blueprints/BPC_Possessable.BPC_Possessable_C")))

(event `/Game/Ships/Components/BPI_ShipComponent.CharacterInteract`
  (params (Character :type "/Game/Characters/Blueprints/BP_Character Object Reference") (Secondary :type Boolean))
  (bind _possessable (`self.Possessable`))
  (if Secondary
    (`/Game/Ships/Blueprints/BPC_Possessable.SetAIEnabled` _possessable false)
    (else
      (`/Game/Ships/Blueprints/BPC_Possessable.SetAIEnabled` _possessable true)
      (set `/Game/Characters/AI/AI_Character.Enabled` false (`/Game/Characters/Blueprints/BP_Character.AIController` Character))
      (`KismetSystemLibrary.PrintString` "can noning")
      (`self.K2_AttachToComponent` Character (`self.GetComponentByClass` (`ChildActorComponent.ChildActor` (`self.Cannon`)) "/Script/Engine.SkeletalMeshComponent") "Pitch" "KeepWorld" "KeepWorld" "KeepWorld" true)
      (`CharacterMovementComponent.SetMovementMode` (`Character.CharacterMovement` Character) "MOVE_None" 0))))

(fn `IsAttended`
  (returns (IsAttended :type Boolean))
  (return (`/Game/Ships/Blueprints/BPC_Possessable.AIEnabled` (`self.Possessable`))))

(fn `UserConstructionScript`
  (`parent.UserConstructionScript`))