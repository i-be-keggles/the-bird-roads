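; BP_ShipComponent_Cannon_AI is an AI-operated cannon ship component that wraps a cannon child actor.
; On BeginPlay it enables AI on the child actor's BPC_Possessable component, and its construction script sets that actor's skeletal mesh to the AnimSharingRed material.
; On Die it runs the parent logic, prints a debug message and calls the OnDeath dispatcher.
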(event `self.Die`
  (`parent.Die`)
  (`KismetSystemLibrary.PrintString` "Cannon died")
  (`self.OnDeath`))

(event `self.ReceiveBeginPlay`
  (`parent.ReceiveBeginPlay`)
  (`/Game/Ships/Blueprints/BPC_Possessable.SetAIEnabled` (`self.GetComponentByClass` (`ChildActorComponent.ChildActor` (`self.Cannon`)) "/Game/Ships/Blueprints/BPC_Possessable.BPC_Possessable_C") true))

(fn `UserConstructionScript`
  (`parent.UserConstructionScript`)
  (`PrimitiveComponent.SetMaterial` (`self.GetComponentByClass` (`ChildActorComponent.ChildActor` (`self.Cannon`)) "/Script/Engine.SkeletalMeshComponent") 0 "/AnimationSharing/AnimSharingRed.AnimSharingRed"))