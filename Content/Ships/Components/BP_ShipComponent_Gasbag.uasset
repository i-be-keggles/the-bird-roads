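; Ship component for an airship gasbag that gains gas leaks as it takes fatal hits and counts as neutralised once twelve accumulate.
; Each Die event adds a BPC_GasLeak to the airship at the previous hit's impact point, oriented along the surface normal and attached to its root.
; RepairComponent removes all tracked leaks and resets the count only when Amount is zero, which is treated as full repair.
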(event `self.Die`
  (bind (_prevhit_bblockinghit _prevhit_binitialoverlap _prevhit_time _prevhit_distance _prevhit_location _prevhit_impactpoint _prevhit_normal _prevhit_impactnormal) (`GameplayStatics.BreakHitResult` (`self.PrevHit`)))
  (bind _returnvalue (`|AddComponentByClass` :`self` (`self.Airship`) :`Class` "/Game/Ships/Blueprints/BPC_GasLeak.BPC_GasLeak_C"))
  (`KismetArrayLibrary.Array_Add` (`self.Gas Leaks`) _returnvalue)
  (`SceneComponent.K2_SetWorldTransform` _returnvalue (`KismetMathLibrary.MakeTransform` _prevhit_impactpoint (`KismetMathLibrary.Conv_VectorToRotator` _prevhit_impactnormal)) false true)
  (`SceneComponent.K2_AttachToComponent` _returnvalue (`/Game/Ships/Blueprints/BP_Airship.Root` (`self.Airship`)) "None" "KeepWorld" "KeepWorld" "KeepWorld" true)
  (`/Engine/EditorBlueprintResources/StandardMacros.IncrementInt` (`self.NumLeaks`)))

(event `self.RepairComponent`
  (params (Amount :type Integer))
  (bind _gas_leaks (`self.Gas Leaks`))
  ;[1 1 1] Only on full repair
  (if (== Amount 0)
    (`KismetSystemLibrary.PrintString` "Reparining gasbag")
    (for _array_element _gas_leaks
      (`/Game/Ships/Blueprints/BPC_GasLeak.RemoveLeak` _array_element))
    (`KismetArrayLibrary.Array_Clear` _gas_leaks)
    (set `self.NumLeaks` 0)))

(fn `IsNeutralised`
  (returns (IsNeutralised :type Boolean))
  (return (>= (`self.NumLeaks`) 12)))

(fn `UserConstructionScript`
  (`parent.UserConstructionScript`))