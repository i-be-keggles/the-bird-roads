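; Ship component for an airship helm that a character can man to switch on AI control of the ship.
; BeginPlay links its possessable component to the parent pawn and that pawn's airship AI controller.
; Interacting attaches the character behind the helm and swaps its AI for the possessable's, while secondary interaction reverses this; IsAttended reports that state.
; Tick eases the handles' rotation toward the airship's joystick input.
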(event `self.ReceiveBeginPlay`
  (`parent.ReceiveBeginPlay`)
  (bind _aspawn (cast `Pawn` (`self.GetParentActor`))
    (:`then`
      (set `/Game/Ships/Blueprints/BPC_Possessable.Pawn` _aspawn (`self.BPC_Possessable`))
      (bind _asai_airship (cast `/Game/Ships/AI/AI_Airship` (`AIBlueprintHelperLibrary.GetAIController` _aspawn))
        (:`then`
          (set `/Game/Ships/AI/AI_Possessable.Possessable` (`self.BPC_Possessable`) _asai_airship))
        (:`CastFailed`
          (`KismetSystemLibrary.PrintString` "nairship"))))
    (:`CastFailed`
      (`KismetSystemLibrary.PrintString` "Helm pawn cast failed"))))

(event `self.Die`
  (`parent.Die`))

(event `/Game/Ships/Components/BPI_ShipComponent.CharacterInteract`
  (params (Character :type "/Game/Characters/Blueprints/BP_Character Object Reference") (Secondary :type Boolean))
  (bind _staticmesh (`self.StaticMesh`))
  (if Secondary
    (`/Game/Ships/Blueprints/BPC_Possessable.SetAIEnabled` (`self.BPC_Possessable`) false)
    (set `/Game/Characters/AI/AI_Character.Enabled` true (`/Game/Characters/Blueprints/BP_Character.AIController` Character))
    (`CharacterMovementComponent.SetMovementMode` (`Character.CharacterMovement` Character) "MOVE_Walking" 0)
    (`self.K2_DetachFromActor` Character "KeepWorld" "KeepWorld" "KeepWorld")
    (else
      (`/Game/Ships/Blueprints/BPC_Possessable.SetAIEnabled` (`self.BPC_Possessable`) true)
      (set `/Game/Characters/AI/AI_Character.Enabled` false (`/Game/Characters/Blueprints/BP_Character.AIController` Character))
      (`self.K2_AttachToComponent` Character (`self.StaticMesh`) "None" "KeepWorld" "KeepWorld" "KeepWorld" false)
      (`CharacterMovementComponent.SetMovementMode` (`Character.CharacterMovement` Character) "MOVE_None" 0)
      (`self.K2_SetActorLocation` Character (+ (`SceneComponent.K2_GetComponentLocation` _staticmesh) (* (`SceneComponent.GetForwardVector` _staticmesh) (`KismetMathLibrary.Conv_DoubleToVector` -80.0)) (* (`SceneComponent.GetUpVector` _staticmesh) (`KismetMathLibrary.Conv_DoubleToVector` 85.0))) false false))))

(event `self.ReceiveTick`
  (params (DeltaSeconds :type "Float (single-precision)"))
  (bind _handles (`self.Handles`))
  (bind (_joystick_x _joystick_y _joystick_z) (`KismetMathLibrary.BreakVector` (`/Game/Ships/Blueprints/BP_Airship.JoyStick` (`self.Airship`))))
  (`SceneComponent.K2_SetRelativeRotation` _handles (`KismetMathLibrary.RLerp` (`SceneComponent.RelativeRotation` _handles) (`KismetMathLibrary.MakeRotator` (* _joystick_z 30.0 -1.0) (* _joystick_y 30.0 -1.0) (* _joystick_x 30.0)) (* DeltaSeconds 5.0)) false false))

(fn `IsAttended`
  (returns (IsAttended :type Boolean))
  (return (`/Game/Ships/Blueprints/BPC_Possessable.AIEnabled` (`self.BPC_Possessable`))))

(fn `UserConstructionScript`
  (`parent.UserConstructionScript`))