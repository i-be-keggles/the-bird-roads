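; Airship propellor component that animates spin with forward input and responds to destruction and repair.
; A looping half-second timer feeds the Airship's forward input into the propellor AnimBP's spin multiplier, defaulting to 1 without a valid Airship.
; Death zeroes the target spin rate and any repair call restores the rate cached at BeginPlay.
; Both then refresh the Airship's PropellorRatio.
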(event `self.ReceiveBeginPlay`
  (`parent.ReceiveBeginPlay`)
  (bind _asabp_propellor (cast `/Game/Ships/Prototypes/BlimpPrototype/Propellor/ABP_Propellor` (`SkeletalMeshComponent.GetAnimInstance` (`self.SkeletalMesh`))))
  (bind _output_get (set `self.AnimBP` _asabp_propellor))
  (set `self.OgSpinRate` (`/Game/Ships/Prototypes/BlimpPrototype/Propellor/ABP_Propellor.TargetSpinRate` _output_get))
  (`KismetSystemLibrary.K2_SetTimerDelegate` (delegate `UpdateSpinSpeed`) 0.5 true))

(event `UpdateSpinSpeed`
  (bind _animbp (`self.AnimBP`))
  (bind _airship (`self.Airship`))
  (`/Engine/EditorBlueprintResources/StandardMacros.IsValid` _airship
    (:`Is Valid`
      (bind _forwardinput (`/Game/Ships/Blueprints/BPI_Airship.GetForwardInput` _airship))
      (set `/Game/Ships/Prototypes/BlimpPrototype/Propellor/ABP_Propellor.SpinrateMultiplier` _forwardinput _animbp))
    (:`Is Not Valid`
      (set `/Game/Ships/Prototypes/BlimpPrototype/Propellor/ABP_Propellor.SpinrateMultiplier` 1.0 _animbp))))

(event `/Game/Ships/Components/BPI_ShipComponent.TakeDamage`
  (params (Amount :type Integer) (Hit :type "HitResult Structure"))
  (`parent.TakeDamage` Amount Hit))

(event `self.Die`
  (bind _airship (`self.Airship`))
  (`parent.Die`)
  (set `/Game/Ships/Prototypes/BlimpPrototype/Propellor/ABP_Propellor.TargetSpinRate` 0.0 (`self.AnimBP`))
  (bind _ratio (`/Game/Ships/Blueprints/BP_Airship.GetPropellorRatio` _airship))
  (set `/Game/Ships/Blueprints/BP_Airship.PropellorRatio` _ratio _airship))

(event `self.RepairComponent`
  (params (Amount :type Integer))
  (bind _airship (`self.Airship`))
  (`parent.RepairComponent` Amount)
  (set `/Game/Ships/Prototypes/BlimpPrototype/Propellor/ABP_Propellor.TargetSpinRate` (`self.OgSpinRate`) (`self.AnimBP`))
  (bind _ratio (`/Game/Ships/Blueprints/BP_Airship.GetPropellorRatio` _airship))
  (set `/Game/Ships/Blueprints/BP_Airship.PropellorRatio` _ratio _airship))

(fn `UserConstructionScript`
  (`parent.UserConstructionScript`))