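; BP_Cannon is a player-controlled ship cannon that aims by pitch and yaw and fires shells.
; Input accumulates clamped angles, with unlimited yaw when its limit is zero, and passes them to ABP_Cannon to animate the mesh.
; Camera and barrel attach to the Pitch socket so they follow the aim.
; Firing spawns BP_CannonShell at the barrel with set damage, gated by a delay cooldown.
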(event `self.ReceiveBeginPlay`
  (`|ExecutionSequence`
    (:`then_0`
      ;[1 1 1] Animate
      (bind _asabp_cannon (cast `/Game/Ships/Weapons/ABP_Cannon` (`SkeletalMeshComponent.GetAnimInstance` (`self.SkeletalMesh`))))
      (set `self.ABP` _asabp_cannon))
    (:`then_1`
      ;[1 1 1] Link components to barrel
      (`SceneComponent.K2_AttachToComponent` (`self.Camera`) (`self.SkeletalMesh`) "Pitch" "KeepWorld" "KeepWorld" "KeepWorld" false)
      (`SceneComponent.K2_AttachToComponent` (`self.Barrel`) (`self.SkeletalMesh`) "Pitch" "KeepWorld" "KeepWorld" "KeepWorld" false))))

(event `Pitch`
  (params (Change :type "Float (double-precision)"))
  (bind (_limits_x _limits_y _limits_z) (`KismetMathLibrary.BreakVector` (`self.Limits`)))
  (bind _output_get (set `self.PitchValue` (`KismetMathLibrary.FClamp` (+ Change (`self.PitchValue`)) _limits_y _limits_z)))
  (set `/Game/Ships/Weapons/ABP_Cannon.Pitch` _output_get (`self.ABP`)))

(event `EnhancedInput|/Game/Ships/Input/IA_PitchYaw`
  (params (ActionValue :type "Vector2D Structure") (ElapsedSeconds :type "Float (double-precision)") (TriggeredSeconds :type "Float (double-precision)") (InputAction :type "InputAction Object Reference" :default "/Game/Ships/Input/IA_PitchYaw.IA_PitchYaw"))
  (:`Triggered`
    (`self.Pitch` ActionValue_Y)
    (`self.Yaw` ActionValue_X)))

(event `EnhancedInput|/Game/Player/Input/Actions/IA_Attack`
  (params (ActionValue :type Boolean) (ElapsedSeconds :type "Float (double-precision)") (TriggeredSeconds :type "Float (double-precision)") (InputAction :type "InputAction Object Reference" :default "/Game/Player/Input/Actions/IA_Attack.IA_Attack"))
  (:`Triggered`
    (if ActionValue
      (`self.Fire`))))

(event `Yaw`
  (params (Change :type "Float (double-precision)"))
  (bind _limits_x (`KismetMathLibrary.BreakVector` (`self.Limits`)))
  (bind _returnvalue (+ Change (`self.YawValue`)))
  (bind _output_get (set `self.YawValue` (select `bool` (== _limits_x 0.0) :`false` (`KismetMathLibrary.FClamp` _returnvalue (* _limits_x -1.0) _limits_x) :`true` _returnvalue)))
  (set `/Game/Ships/Weapons/ABP_Cannon.Yaw` _output_get (`self.ABP`)))

(event `Fire`
  (if (`self.CanFire`)
    (bind _returnvalue (`|SpawnActorFromClass` "/Game/Ships/Weapons/BP_CannonShell.BP_CannonShell_C" (`SceneComponent.K2_GetComponentToWorld` (`self.Barrel`)) "Undefined" "MultiplyWithRoot" null null))
    (set `/Game/Ships/Weapons/BP_CannonShell.Damage` (`self.Damage`) _returnvalue)
    (set `self.CanFire` false)
    (`KismetSystemLibrary.Delay` (`self.FireDelay`))
    (set `self.CanFire` true)))

(fn `UserConstructionScript`)