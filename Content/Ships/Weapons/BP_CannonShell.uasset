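; Physics-driven ship cannon shell that launches forward, turns to follow its velocity and explodes on impact or timeout.
; After a short arming delay, a per-tick sphere trace along the next frame's movement catches hits alongside component hit events.
; Explode sends damage messages to overlapped owners, tracked to skip repeats, and pushes physics bodies away.
; It also attaches a blast decal, plays Niagara and sound effects, then hides and later destroys the shell.
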(event `self.ReceiveBeginPlay`
  (bind _cannonshell (`self.CannonShell`))
  (`PrimitiveComponent.SetPhysicsLinearVelocity` _cannonshell (* (`SceneComponent.GetForwardVector` _cannonshell) (`self.Force`)) false "None")
  (`KismetSystemLibrary.Delay` 0.1)
  (set `self.Primed` true)
  (`KismetSystemLibrary.Delay` 10.0)
  (`self.Explode`))

(event `self.ReceiveTick`
  (params (DeltaSeconds :type "Float (single-precision)"))
  (bind _cannonshell (`self.CannonShell`))
  (bind _cannonshell_2 (`self.CannonShell`))
  (bind _returnvalue (`SceneComponent.K2_GetComponentLocation` _cannonshell_2))
  (`SceneComponent.K2_SetWorldRotation` _cannonshell (`KismetMathLibrary.FindLookAtRotation` (`KismetMathLibrary.Vector_Zero`) (`SceneComponent.GetComponentVelocity` _cannonshell)) false false)
  (if (`self.Primed`)
    (bind (_outhit _returnvalue_2) (`KismetSystemLibrary.SphereTraceSingle` _returnvalue (+ _returnvalue (* (`SceneComponent.GetComponentVelocity` _cannonshell_2) DeltaSeconds)) 10.0 "TraceTypeQuery1"))
    (set `self.Hit` _outhit)
    (if _returnvalue_2
      (`SceneComponent.K2_SetWorldLocation` (`self.CannonShell`) (`.ImpactPoint` (`GameplayStatics.BreakHitResult` _outhit)) false true)
      (`self.Explode`))))

(event `self.CannonShell.OnComponentHit`
  (params (HitComponent :type "PrimitiveComponent Object Reference") (OtherActor :type "Actor Object Reference") (OtherComp :type "PrimitiveComponent Object Reference") (NormalImpulse :type "Vector Structure") (Hit :type "HitResult Structure (by ref)"))
  (`KismetSystemLibrary.PrintString` "HIT")
  (if (`self.Primed`)
    (`self.Explode`)))

(event `Explode`
  (bind _hit (`self.Hit`))
  (bind _cannonshell (`self.CannonShell`))
  (bind _damage (`self.Damage`))
  (bind _returnvalue (`SceneComponent.K2_GetComponentLocation` (`self.CannonShell`)))
  (bind (_bblockinghit _binitialoverlap _time _distance _location _impactpoint _normal _impactnormal _physmat _hitactor _hitcomponent) (`GameplayStatics.BreakHitResult` _hit))
  (bind (_returnvalue_roll _returnvalue_pitch _returnvalue_yaw) (`KismetMathLibrary.BreakRotator` (`KismetMathLibrary.Conv_VectorToRotator` _normal)))
  (`|ExecutionSequence`
    (:`then_0`
      ;[1 1 1] Damage
      (`|ExecutionSequence`
        (:`then_0`
          (bind _outcomponents (`KismetSystemLibrary.SphereOverlapComponents` _location (`self.ExplosionRadius`) (`|MakeArray` "ObjectTypeQuery8" "ObjectTypeQuery3" "ObjectTypeQuery2" "ObjectTypeQuery1" "ObjectTypeQuery4" :!type "EObjectTypeQuery Enum")))
          (for _array_element _outcomponents
            (bind _returnvalue_2 (`ActorComponent.GetOwner` _array_element))
            (if (not (`KismetArrayLibrary.Array_Contains` (`self.DamagedActors`) _returnvalue_2))
              (message `/Game/Ships/Components/BPI_ShipComponent.TakeDamage` _returnvalue_2 _damage _hit)
              (`KismetArrayLibrary.Array_Add` (`self.DamagedActors`) _returnvalue_2)
              (if (`SceneComponent.IsSimulatingPhysics` _array_element "None")
                (`PrimitiveComponent.AddForce` _array_element (* (`KismetMathLibrary.Normal` (- (`SceneComponent.K2_GetComponentLocation` _array_element) _location)) 10000000.0) "None" false))
              (message `/Game/Characters/Blueprints/BPI_Lifecycle.TakeDamage` _returnvalue_2 _damage (struct) null))))
        (:`then_1`
          (bind _returnvalue_3 (`|SpawnActorFromClass` "/Script/Engine.DecalActor" (`KismetMathLibrary.MakeTransform` _impactpoint (`KismetMathLibrary.MakeRotator` 0.0 (+ _returnvalue_pitch 90.0) _returnvalue_yaw)) "Undefined" "MultiplyWithRoot" null null))
          (`DecalComponent.SetDecalMaterial` (`DecalActor.Decal` _returnvalue_3) "/Game/FX/Materials/M_CannonBlastDecal.M_CannonBlastDecal")
          (`self.K2_AttachToComponent` _returnvalue_3 _hitcomponent "None" "KeepWorld" "KeepWorld" "KeepWorld" true))))
    (:`then_1`
      ;[1 1 1] FX
      (`NiagaraFunctionLibrary.SpawnSystemAtLocation` "/Game/FX/NiagaraSystems/NS_Explosion.NS_Explosion" _returnvalue)
      (bind _returnvalue_4 (`GameplayStatics.SpawnSoundAtLocation` "/Game/SFX/Metasounds/MS_BasicSound.MS_BasicSound" _returnvalue (struct) 1.0 1.0 0.0 "/Game/SFX/Attenuation/SA_AirshipLongAttenuation.SA_AirshipLongAttenuation" null))
      (`AudioComponent.SetWaveParameter` _returnvalue_4 "Sound" "/Game/SFX/WaveAssets/Explosion.Explosion")
      (`SceneComponent.SetHiddenInGame` _cannonshell true false)
      (`PrimitiveComponent.SetSimulatePhysics` _cannonshell false)
      (`PrimitiveComponent.SetCollisionEnabled` _cannonshell "NoCollision")
      (set `self.Primed` false)
      (`KismetSystemLibrary.Delay` 5.0)
      (`self.K2_DestroyActor`))))

(fn `UserConstructionScript`)